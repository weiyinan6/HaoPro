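; PC_Game is the game's player controller, handling input mapping contexts, the HUD and Narrative dialogue.
; On BeginPlay it adds the rolling drone and menu Enhanced Input contexts, creates the WBP_NHUD widget and starts a test dialogue.
; When the Narrative component reports a dialogue has begun, the HUD's nested Narrative HUD opens the dialogue menu.
; RegisterContext and DeRegisterContext wrap adding and removing mapping contexts.
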(event `self.ReceiveBeginPlay`
  (bind _returnvalue (subsystem `EnhancedInputLocalPlayerSubsystem`))
  (`EnhancedInputSubsystemInterface.AddMappingContext` _returnvalue "/Game/ThirdPerson/Input/RollingDrone/IMC_RollingDrone.IMC_RollingDrone" 0 (struct))
  (`EnhancedInputSubsystemInterface.AddMappingContext` _returnvalue "/Game/ThirdPerson/Input/Inventory/IMC_MenuContent.IMC_MenuContent" 0 (struct))
  (bind _returnvalue_2 (`|CreateWidget` "/Game/Narrative/WBP_NHUD.WBP_NHUD_C"))
  (bind _output_get (set `self.NHUD` _returnvalue_2))
  (`UserWidget.AddToViewport` _output_get 0)
  (`NarrativeComponent.BeginDialogue` (`self.Narrative`) "/Game/Narrative/Test.Test_C" "None"))

(event `self.Narrative.OnDialogueBegan`
  (params (Dialogue :type "Dialogue Object Reference"))
  (`/NarrativeCommonUI/Widgets/WBP_NarrativeHUD.OpenMenu` (`/Game/Narrative/WBP_NHUD.WBP_NarrativeHUD` (`self.NHUD`)) "/Narrative/NarrativeUI/Widgets/W_NarrativeMenu_Dialogue.W_NarrativeMenu_Dialogue_C"))

(fn `DeRegisterContext`
  (params (MappingContext :type "InputMappingContext Object Reference"))
  (`EnhancedInputSubsystemInterface.RemoveMappingContext` (subsystem `EnhancedInputLocalPlayerSubsystem`) MappingContext (struct)))

(fn `RegisterContext`
  (params (MappingContext :type "InputMappingContext Object Reference"))
  (`EnhancedInputSubsystemInterface.AddMappingContext` (subsystem `EnhancedInputLocalPlayerSubsystem`) MappingContext 0 (struct)))

(fn `UserConstructionScript`)