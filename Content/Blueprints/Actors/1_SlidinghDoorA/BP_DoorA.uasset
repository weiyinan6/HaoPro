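; Sliding sci-fi door that the player toggles, or locks with a key card to block enemies.
; Locking consumes the card, shuts the door, turns the light red and shows a card on the player's side, tracked by overlap volumes.
; Interacting refunds the card and unlocks; unlocked toggles emit AI noise, while UniqueLocked refuses interaction.
; AI entering the box opens unlocked doors; prompt-widget and auto-close logic is unwired.
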(event `/Game/Blueprints/Interface/BPI_Interact.LockDoor`
  (if (`self.Locked`)
    (`KismetSystemLibrary.PrintString` "AlreadyLocked")
    (else
      (bind _asbp_player_character_may (cast `/Game/ThirdPerson/Blueprints/BP_PlayerCharacter_May` (`GameplayStatics.GetPlayerCharacter` 0)))
      (bind _ac_inventory (`/Game/ThirdPerson/Blueprints/BP_PlayerCharacter_May.AC_Inventory` _asbp_player_character_may))
      (if (`/Game/Inventory/Inventory_CQB/AC_Inventory_May.IsItemAlreadyInInventory?` _ac_inventory (make `/Game/Inventory/Inventory_CQB/S_InventoryItemData` "Key Cards" "NewEnumerator0" "" 0 null))
        (`/Game/Inventory/Inventory_CQB/AC_Inventory_May.UseItem` _ac_inventory (`self.KeyCard`))
        (set `self.Locked` true)
        (`KismetSystemLibrary.PrintString` "DoorLocked!")
        (`LightComponent.SetLightColor` (`self.SpotLight`) (struct :`R` 1.0 :`B` 0.064521 :`A` 1.0) true)
        (`self.CloseDoor`)
        (if (`self.OnSideA`)
          (`SceneComponent.SetVisibility` (`self.KeyA`) true false)
          (else
            (`SceneComponent.SetVisibility` (`self.KeyB`) true false)))
        (else
          (`KismetSystemLibrary.PrintString` "NoKeycard!"))))))

(event `self.SideA.OnComponentBeginOverlap`
  (params (OverlappedComponent :type "PrimitiveComponent Object Reference") (OtherActor :type "Actor Object Reference") (OtherComp :type "PrimitiveComponent Object Reference") (OtherBodyIndex :type Integer) (bFromSweep :type Boolean) (SweepResult :type "HitResult Structure (by ref)"))
  (cast `/Game/ThirdPerson/Blueprints/BP_PlayerCharacter_May` OtherActor)
  (set `self.OnSideA` true)
  (set `self.OnSide B` false))

(event `/Game/Blueprints/Interface/BPI_Interact.Interact`
  (params (Actor :type "Actor Object Reference"))
  (`self.ToggleDoor`))

(event `self.SideB.OnComponentBeginOverlap`
  (params (OverlappedComponent :type "PrimitiveComponent Object Reference") (OtherActor :type "Actor Object Reference") (OtherComp :type "PrimitiveComponent Object Reference") (OtherBodyIndex :type Integer) (bFromSweep :type Boolean) (SweepResult :type "HitResult Structure (by ref)"))
  (cast `/Game/ThirdPerson/Blueprints/BP_PlayerCharacter_May` OtherActor)
  (set `self.OnSide B` true)
  (set `self.OnSideA` false))

(event `ToggleDoor`
  (if (`self.UniqueLocked`)
    (`KismetSystemLibrary.PrintString` "Level 2 Card Required")
    (else
      (if (`self.Locked`)
        (bind _asbp_player_character_may (cast `/Game/ThirdPerson/Blueprints/BP_PlayerCharacter_May` (`GameplayStatics.GetPlayerCharacter` 0)))
        (`/Game/Inventory/Inventory_CQB/AC_Inventory_May.AddItemToInventory` (`/Game/ThirdPerson/Blueprints/BP_PlayerCharacter_May.AC_Inventory` _asbp_player_character_may) (make `/Game/Inventory/Inventory_CQB/S_InventoryItemData` "Key Cards" "NewEnumerator0" "" 1 "/Game/Inventory/Inventory_CQB/A_StaticMesh_KeyItems_KeyCard.A_StaticMesh_KeyItems_KeyCard_C"))
        (set `self.Locked` false)
        (`LightComponent.SetLightColor` (`self.SpotLight`) (struct :`G` 1.0 :`B` 0.576471 :`A` 1.0) true)
        (`SceneComponent.SetVisibility` (`self.KeyA`) false false)
        (`SceneComponent.SetVisibility` (`self.KeyB`) false false)
        (else
          (`self.MakeNoise` 5.0 null (`SceneComponent.K2_GetComponentLocation` (`self.StaticMesh1`)) 10.0)))
      (if (`self.Opened?`)
        (`self.CloseDoor`)
        (else
          (`self.DoorOpen`))))))

(event `DoorOpen`
  (`SceneComponent.SetVisibility` (`self.KeyB`) false false)
  (`GameplayStatics.SpawnSoundAtLocation` "/Game/SFX/Doors_SciFi/Cues/Door_Scifi_Small_01_Open_Cue.Door_Scifi_Small_01_Open_Cue" (`self.K2_GetActorLocation`) (struct) 1.0 1.0 0.0 null null)
  (`KismetSystemLibrary.MoveComponentTo` (`self.StaticMesh1`) (-111.666142 -0.194965 -5.243243) (struct) true true 1.0)
  (set `self.Opened?` true))

(event `CloseDoor`
  (`GameplayStatics.SpawnSoundAtLocation` "/Game/SFX/Doors_SciFi/Cues/Door_Scifi_Small_01_Close_Cue.Door_Scifi_Small_01_Close_Cue" (`self.K2_GetActorLocation`) (struct) 1.0 1.0 0.0 null null)
  (`KismetSystemLibrary.MoveComponentTo` (`self.StaticMesh1`) (-1.368197 -0.194965 -5.243243) (struct) true true 1.0)
  (set `self.Opened?` false))

(event `self.Box.OnComponentBeginOverlap`
  (params (OverlappedComponent :type "PrimitiveComponent Object Reference") (OtherActor :type "Actor Object Reference") (OtherComp :type "PrimitiveComponent Object Reference") (OtherBodyIndex :type Integer) (bFromSweep :type Boolean) (SweepResult :type "HitResult Structure (by ref)"))
  (`|ExecutionSequence`
    (:`then_0`
      (cast `/Game/ThirdPerson/Blueprints/BP_PlayerCharacter_May` OtherActor))
    (:`then_1`
      (cast `/Game/AIBehaviorSystem/Blueprint/AI/BP_AI_Base` OtherActor)
      (if (`self.Locked`)
        (`KismetSystemLibrary.PrintString` "EnemyBlocked")
        (else
          (`self.DoorOpen`))))))

(event `self.Box.OnComponentEndOverlap`
  (params (OverlappedComponent :type "PrimitiveComponent Object Reference") (OtherActor :type "Actor Object Reference") (OtherComp :type "PrimitiveComponent Object Reference") (OtherBodyIndex :type Integer))
  (`|ExecutionSequence`
    (:`then_0`
      (cast `/Game/ThirdPerson/Blueprints/BP_PlayerCharacter_May` OtherActor))))

(fn `CanBeAssassinated?`
  (returns (`CanAssassnate?` :type Boolean))
  (return false))

(fn `UserConstructionScript`)