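; BP_Door is a sliding door the player can toggle, or lock with a keycard to block the monster.
; Locking spends a keycard, closes the door and turns its light red; interacting while locked refunds the card, turns it green and toggles the door silently.
; Toggling an unlocked door emits noise.
; Box overlaps show the player's prompt, open unlocked doors for Monster_NBC, and close the door shortly after the player leaves.
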(event `/Game/Blueprints/Interface/BPI_Interact.LockDoor`
  (if (`self.Locked`)
    (`KismetSystemLibrary.PrintString` "AlreadyLocked")
    (else
      (bind _asbp_player_character_1 (cast `/Game/ThirdPerson/Blueprints/BP_PlayerCharacter1` (`GameplayStatics.GetPlayerCharacter` 0)))
      (bind _keycardsamount (`/Game/ThirdPerson/Blueprints/BP_PlayerCharacter1.KeycardsAmount` _asbp_player_character_1))
      (if (> _keycardsamount 0)
        (`/Engine/EditorBlueprintResources/StandardMacros.DecrementInt` _keycardsamount
          (:`  `
            (set `self.Locked` true)
            (`KismetSystemLibrary.PrintString` "DoorLocked!")
            (`LightComponent.SetLightColor` (`self.SpotLight`) (struct :`R` 1.0 :`B` 0.064521 :`A` 1.0) true)
            (`self.CloseDoor`)))
        (else
          (`KismetSystemLibrary.PrintString` "NoKeycard!"))))))

(event `/Game/Blueprints/Interface/BPI_Interact.Interact`
  (`self.ToggleDoor`))

(event `ToggleDoor`
  (if (`self.Locked`)
    (bind _asbp_player_character_1 (cast `/Game/ThirdPerson/Blueprints/BP_PlayerCharacter1` (`GameplayStatics.GetPlayerCharacter` 0)))
    (bind _result (`/Engine/EditorBlueprintResources/StandardMacros.IncrementInt` (`/Game/ThirdPerson/Blueprints/BP_PlayerCharacter1.KeycardsAmount` _asbp_player_character_1))
      (:`  `
        (set `/Game/ThirdPerson/Blueprints/BP_PlayerCharacter1.KeycardsAmount` _result _asbp_player_character_1)
        (set `self.Locked` false)
        (`LightComponent.SetLightColor` (`self.SpotLight`) (struct :`G` 1.0 :`B` 0.576471 :`A` 1.0) true)))
    (else
      (`self.MakeNoise` 5.0 null (`SceneComponent.K2_GetComponentLocation` (`self.StaticMesh1`)) 10.0)))
  (if (`self.Opened?`)
    (`self.CloseDoor`)
    (else
      (`self.DoorOpen`))))

(event `DoorOpen`
  (`KismetSystemLibrary.MoveComponentTo` (`self.StaticMesh1`) (0.0 128.0 0.0) (struct) true true 1.0)
  (set `self.Opened?` true))

(event `CloseDoor`
  (`KismetSystemLibrary.MoveComponentTo` (`self.StaticMesh1`) (0.0 44.683886 0.0) (struct) true true 1.0)
  (set `self.Opened?` false))

(event `self.Box.OnComponentBeginOverlap`
  (params (OverlappedComponent :type "PrimitiveComponent Object Reference") (OtherActor :type "Actor Object Reference") (OtherComp :type "PrimitiveComponent Object Reference") (OtherBodyIndex :type Integer) (bFromSweep :type Boolean) (SweepResult :type "HitResult Structure (by ref)"))
  (`|ExecutionSequence`
    (:`then_0`
      (cast `/Game/ThirdPerson/Blueprints/BP_PlayerCharacter1` OtherActor)
      (bind _returnvalue (`|CreateWidget` "/Game/Blueprints/Widget/BPW_PeekOrInteractrPrompt.BPW_PeekOrInteractrPrompt_C"))
      (if (`self.Locked`)
        (`TextBlock.SetText` (`/Game/Blueprints/Widget/BPW_PeekOrInteractrPrompt.OpenClose` _returnvalue) "E 解锁"))
      (`UserWidget.AddToViewport` _returnvalue 0))
    (:`then_1`
      (cast `/Game/MonsterAi_Kit/Monster_NBC` OtherActor)
      (if (`self.Locked`)
        (`KismetSystemLibrary.PrintString` "EnemyBlocked")
        (else
          (`self.DoorOpen`))))))

(event `self.Box.OnComponentEndOverlap`
  (params (OverlappedComponent :type "PrimitiveComponent Object Reference") (OtherActor :type "Actor Object Reference") (OtherComp :type "PrimitiveComponent Object Reference") (OtherBodyIndex :type Integer))
  (`|ExecutionSequence`
    (:`then_0`
      (cast `/Game/ThirdPerson/Blueprints/BP_PlayerCharacter1` OtherActor)
      (`Widget.RemoveFromParent` (stale `self.Box.OnComponentBeginOverlap` _returnvalue))
      (`KismetSystemLibrary.Delay` 2.0)
      (`self.CloseDoor`))))

(fn `UserConstructionScript`)