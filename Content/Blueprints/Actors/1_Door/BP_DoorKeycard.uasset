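; Sliding keycard door that opens or closes on Interact if the player holds at least one keycard, otherwise prints "Locked".
; Toggling emits a noise at the door, then eases the mesh sideways with MoveComponentTo.
; Peek flip-flops the view between the door's camera and the player.
; A trigger box shows the peek/interact prompt to the player and opens the door directly for Monster_NBC, bypassing keycard check and noise.
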(event `self.Interact`
  (bind _asbp_third_person_character (cast `/Game/ThirdPerson/Blueprints/BP_ThirdPersonCharacter` (`GameplayStatics.GetPlayerCharacter` 0)))
  (if (> (`/Game/ThirdPerson/Blueprints/BP_ThirdPersonCharacter.KeycardsAmount` _asbp_third_person_character) 0)
    (`self.ToggleDoor`)
    (else
      (`KismetSystemLibrary.PrintString` "Locked"))))

(event `ToggleDoor`
  (`self.MakeNoise` 5.0 null (`SceneComponent.K2_GetComponentLocation` (`self.StaticMesh1`)) 10.0)
  (if (`self.Opened?`)
    (`self.CloseDoor`)
    (else
      (`self.DoorOpen`))))

(event `DoorOpen`
  (`KismetSystemLibrary.MoveComponentTo` (`self.StaticMesh1`) (0.0 128.0 0.0) (struct) true true 1.0)
  (set `self.Opened?` true))

(event `self.Peek`
  (`/Engine/EditorBlueprintResources/StandardMacros.FlipFlop`
    (:`A`
      (`PlayerController.SetViewTargetWithBlend` (`GameplayStatics.GetPlayerController` 0) (`ActorComponent.GetOwner` (`self.Camera`)) 0.5 "VTBlend_Linear" 1.0 false))
    (:`B`
      (bind _asbp_third_person_character (cast `/Game/ThirdPerson/Blueprints/BP_ThirdPersonCharacter` (`GameplayStatics.GetPlayerCharacter` 0)))
      (`PlayerController.SetViewTargetWithBlend` (`GameplayStatics.GetPlayerController` 0) _asbp_third_person_character 0.5 "VTBlend_Linear" 1.0 false))))

(event `CloseDoor`
  (`KismetSystemLibrary.MoveComponentTo` (`self.StaticMesh1`) (0.0 44.683886 0.0) (struct) true true 1.0)
  (set `self.Opened?` false))

(event `self.Box.OnComponentBeginOverlap`
  (params (OverlappedComponent :type "PrimitiveComponent Object Reference") (OtherActor :type "Actor Object Reference") (OtherComp :type "PrimitiveComponent Object Reference") (OtherBodyIndex :type Integer) (bFromSweep :type Boolean) (SweepResult :type "HitResult Structure (by ref)"))
  (`|ExecutionSequence`
    (:`then_0`
      (cast `/Game/ThirdPerson/Blueprints/BP_ThirdPersonCharacter` OtherActor)
      (bind _returnvalue (`|CreateWidget` "/Game/Blueprints/Widget/BPW_PeekOrInteractrPrompt.BPW_PeekOrInteractrPrompt_C"))
      (`UserWidget.AddToViewport` _returnvalue 0))
    (:`then_1`
      (cast `/Game/MonsterAi_Kit/Monster_NBC` OtherActor)
      (`self.DoorOpen`))))

(event `self.Box.OnComponentEndOverlap`
  (params (OverlappedComponent :type "PrimitiveComponent Object Reference") (OtherActor :type "Actor Object Reference") (OtherComp :type "PrimitiveComponent Object Reference") (OtherBodyIndex :type Integer))
  (`|ExecutionSequence`
    (:`then_0`
      (cast `/Game/ThirdPerson/Blueprints/BP_ThirdPersonCharacter` OtherActor)
      (`Widget.RemoveFromParent` (stale `self.Box.OnComponentBeginOverlap` _returnvalue)))))

(fn `UserConstructionScript`)