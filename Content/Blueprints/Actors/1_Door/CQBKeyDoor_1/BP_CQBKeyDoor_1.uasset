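; Sliding keycard door that the player toggles, and that lets Monster_NBC through unless it is locked.
; Locking consumes a key card, closes the door and shows SideABox if OnSideA is set; unlocking returns the card.
; MoveComponentTo slides the panel, and toggling an unlocked door makes noise.
; The trigger box shows the player an interact prompt, auto-opens for monsters, and closes the door shortly after the player leaves.
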(event `self.LockDoor`
  (if (`self.Locked`)
    (`KismetSystemLibrary.PrintString` "AlreadyLocked")
    (else
      (bind _asbp_player_character_may (cast `/Game/ThirdPerson/Blueprints/BP_PlayerCharacter_May` (`GameplayStatics.GetPlayerCharacter` 0)))
      (bind _ac_inventory (`/Game/ThirdPerson/Blueprints/BP_PlayerCharacter_May.AC_Inventory` _asbp_player_character_may))
      (if (`/Game/Inventory/Inventory_Shooter/AC_Inventory.IsItemAlreadyInInventory?` _ac_inventory (make `/Game/Inventory/Inventory_Shooter/S_ItemData` "Key Cards"))
        (`/Game/Inventory/Inventory_Shooter/AC_Inventory.Remove Single Item Without Spawn` _ac_inventory (`self.KeyCard`))
        (set `self.Locked` true)
        (`KismetSystemLibrary.PrintString` "DoorLocked!")
        (`self.CloseDoor`)
        (if (`self.OnSideA`)
          (`SceneComponent.SetVisibility` (`self.SideABox`) true false)
          (else
            (`SceneComponent.SetVisibility` (`self.SideABox`) false false)))
        (else
          (`KismetSystemLibrary.PrintString` "NoKeycard!"))))))

(event `self.SideA.OnComponentBeginOverlap`
  (params (OverlappedComponent :type "PrimitiveComponent Object Reference") (OtherActor :type "Actor Object Reference") (OtherComp :type "PrimitiveComponent Object Reference") (OtherBodyIndex :type Integer) (bFromSweep :type Boolean) (SweepResult :type "HitResult Structure (by ref)"))
  (cast `/Game/ThirdPerson/Blueprints/BP_PlayerCharacter_May` OtherActor)
  (set `self.OnSideA` true))

(event `RollingDroneInteract`)

(event `self.Interact`
  (`self.ToggleDoor`))

(event `ToggleDoor`
  (if (`self.Locked`)
    (bind _asbp_player_character_may (cast `/Game/ThirdPerson/Blueprints/BP_PlayerCharacter_May` (`GameplayStatics.GetPlayerCharacter` 0)))
    (`/Game/Inventory/Inventory_Shooter/AC_Inventory.AddItemToInventory` (`/Game/ThirdPerson/Blueprints/BP_PlayerCharacter_May.AC_Inventory` _asbp_player_character_may) (make `/Game/Inventory/Inventory_Shooter/S_ItemData` "Key Cards" "NewEnumerator0" "" 1 "/Game/Inventory/Inventory_Shooter/A_StaticMesh_KeyItems_KeyCard.A_StaticMesh_KeyItems_KeyCard_C"))
    (set `self.Locked` false)
    (else
      (`self.MakeNoise` 5.0 null (`SceneComponent.K2_GetComponentLocation` (`self.DoorSliding`)) 10.0)))
  (if (`self.Opened?`)
    (`self.CloseDoor`)
    (else
      (`self.DoorOpen`))))

(event `DoorOpen`
  (`SceneComponent.SetVisibility` (`self.SideABox`) false false)
  (`KismetSystemLibrary.MoveComponentTo` (`self.DoorSliding`) (1118.172503 -1181.286897 1005.508941) (struct :`Yaw` 90.0) true true 1.0)
  (set `self.Opened?` true)
  (if (`self.Locked`)
    (cast `/Game/ThirdPerson/Blueprints/BP_PlayerCharacter_May` (`GameplayStatics.GetPlayerCharacter` 0))))

(event `CloseDoor`
  (`KismetSystemLibrary.MoveComponentTo` (`self.DoorSliding`) (1118.172503 -17.401317 1005.508931) (struct :`Yaw` 90.0) true true 1.0)
  (set `self.Opened?` false))

(event `self.Box.OnComponentBeginOverlap`
  (params (OverlappedComponent :type "PrimitiveComponent Object Reference") (OtherActor :type "Actor Object Reference") (OtherComp :type "PrimitiveComponent Object Reference") (OtherBodyIndex :type Integer) (bFromSweep :type Boolean) (SweepResult :type "HitResult Structure (by ref)"))
  (`|ExecutionSequence`
    (:`then_0`
      (cast `/Game/ThirdPerson/Blueprints/BP_PlayerCharacter_May` OtherActor)
      (bind _returnvalue (`|CreateWidget` "/Game/Blueprints/Widget/BPW_PeekOrInteractrPrompt.BPW_PeekOrInteractrPrompt_C"))
      (if (`self.Locked`)
        (`TextBlock.SetText` (`/Game/Blueprints/Widget/BPW_PeekOrInteractrPrompt.OpenClose` _returnvalue) "E 解锁"))
      (`UserWidget.AddToViewport` _returnvalue 0))
    (:`then_1`
      (cast `/Game/MonsterAi_Kit/Monster_NBC` OtherActor)
      (if (`self.Locked`)
        (`KismetSystemLibrary.PrintString` "EnemyBlocked")
        (else
          (`self.DoorOpen`))))))

(event `self.Box.OnComponentEndOverlap`
  (params (OverlappedComponent :type "PrimitiveComponent Object Reference") (OtherActor :type "Actor Object Reference") (OtherComp :type "PrimitiveComponent Object Reference") (OtherBodyIndex :type Integer))
  (`|ExecutionSequence`
    (:`then_0`
      (cast `/Game/ThirdPerson/Blueprints/BP_PlayerCharacter_May` OtherActor)
      (`Widget.RemoveFromParent` (stale `self.Box.OnComponentBeginOverlap` _returnvalue))
      (`KismetSystemLibrary.Delay` 5.0)
      (`self.CloseDoor`))))

(fn `UserConstructionScript`)