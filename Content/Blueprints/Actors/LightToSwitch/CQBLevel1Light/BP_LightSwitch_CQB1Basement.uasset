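; Interactable light switch for the CQB1 basement that toggles the level's spotlights between bright and dark, starting flagged as bright.
; The interact input flips the state, plays the switch animation, then after a short delay sets the intensity of every basement spotlight actor.
; It also updates the lamp material parameter collection and the player's NPR brightness and color collection, calling the May character's lighting update so character shading follows the room.
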(event `EnhancedInput|/Game/ThirdPerson/Input/Actions/IA_Interact`
  (params (ActionValue :type Boolean) (ElapsedSeconds :type "Float (double-precision)") (TriggeredSeconds :type "Float (double-precision)") (InputAction :type "InputAction Object Reference" :default "/Game/ThirdPerson/Input/Actions/IA_Interact.IA_Interact"))
  (:`Triggered`
    (`self.SwitchInteract`)))

(event `self.ReceiveBeginPlay`
  ;[1 1 1] Set Bright at beginning
  (bind _outactors (`GameplayStatics.GetAllActorsOfClass` "/Game/ThirdPerson/Blueprints/BP_PlayerCharacter_May.BP_PlayerCharacter_May_C"))
  (for _ _outactors
    (set `self.IsLightBright?` true)))

(event `/Game/Blueprints/Actors/LightToSwitch/CQBLevel1Light/BPI_SwitchInteract.SwitchInteract`
  ;[1 1 1] Switch triggered Light Intensity Change
  (bind _outactors (`GameplayStatics.GetAllActorsOfClass` "/Game/ThirdPerson/Blueprints/BP_PlayerCharacter_May.BP_PlayerCharacter_May_C"))
  (for _array_element _outactors
    (if (`self.IsLightBright?`)
      (set `self.IsLightBright?` false)
      (`/Game/Blueprints/Actors/LightToSwitch/CQBLevel1Light/BPI_SwitchInteract.TurnOffLight`)
      (else
        (set `self.IsLightBright?` true)
        (`self.TurnOnLight`)))))

(event `/Game/Blueprints/Actors/LightToSwitch/CQBLevel1Light/BPI_SwitchInteract.TurnOffLight`
  ;[1 1 1] Switch triggered Light Intensity Change
  ;;[1 1 1] Switch Anm
  (`SkeletalMeshComponent.PlayAnimation` (`self.CQB1LightSwitch`) "/Game/Blueprints/Actors/LightToSwitch/CQBLevel1Light/Anm/ANM_CQB1LightSwitch_LightOnToOff.ANM_CQB1LightSwitch_LightOnToOff" false)
  (`KismetSystemLibrary.Delay` 0.4)
  (bind _outactors (`GameplayStatics.GetAllActorsOfClass` "/Game/Blueprints/Actors/LightToSwitch/CQBLevel1Light/BP_Light_CQB1_Spotlight_Basement.BP_Light_CQB1_Spotlight_Basement_C"))
  (for _array_element _outactors
    (`LightComponent.SetIntensity` (`/Game/Blueprints/Actors/LightToSwitch/CQBLevel1Light/BP_LightToSwitch_SpotLight.SpotLight` _array_element) (`self.Dark Light Intensity_Switch`))
    ;[1 1 1] Light Material
    (`KismetMaterialLibrary.SetScalarParameterValue` "/Game/Blueprints/Actors/LightToSwitch/CQBLevel1Light/MPC_CQBLamp.MPC_CQBLamp" "TexTransition(Bright0 to Dark1)" 1.0)
    ;[0.001042 0.001042 0.001042] NPR Influence
    (`/Game/ThirdPerson/Blueprints/BP_PlayerCharacter_May.CharacterBrightnessNLightColor` (stale `/Game/Blueprints/Actors/LightToSwitch/CQBLevel1Light/BPI_SwitchInteract.SwitchInteract` _array_element))
    (`KismetMaterialLibrary.SetScalarParameterValue` "/Game/Characters/VTGCharacterShader/Player_LightColor.Player_LightColor" "NPRBrightnessOverall" 0.6)
    (`KismetMaterialLibrary.SetVectorParameterValue` "/Game/Characters/VTGCharacterShader/Player_LightColor.Player_LightColor" "NPRColorBlend" (`self.NPRColor_LightBasement`))))

(event `/Game/Blueprints/Actors/LightToSwitch/CQBLevel1Light/BPI_SwitchInteract.TurnOnLight`
  ;[1 1 1] Switch triggered Light Intensity Change
  ;;[1 1 1] Switch Anm
  (`SkeletalMeshComponent.PlayAnimation` (`self.CQB1LightSwitch`) "/Game/Blueprints/Actors/LightToSwitch/CQBLevel1Light/Anm/ANM_CQB1LightSwitch_LightOffToOn.ANM_CQB1LightSwitch_LightOffToOn" false)
  (`KismetSystemLibrary.Delay` 0.2)
  (bind _outactors (`GameplayStatics.GetAllActorsOfClass` "/Game/Blueprints/Actors/LightToSwitch/CQBLevel1Light/BP_Light_CQB1_Spotlight_Basement.BP_Light_CQB1_Spotlight_Basement_C"))
  (for _array_element _outactors
    (`LightComponent.SetIntensity` (`/Game/Blueprints/Actors/LightToSwitch/CQBLevel1Light/BP_LightToSwitch_SpotLight.SpotLight` _array_element) (`self.Bright Light Intensity_Switch`))
    ;[1 1 1] Light Material
    (`KismetMaterialLibrary.SetScalarParameterValue` "/Game/Blueprints/Actors/LightToSwitch/CQBLevel1Light/MPC_CQBLamp.MPC_CQBLamp" "TexTransition(Bright0 to Dark1)")
    ;[0.001042 0.001042 0.001042] NPR Influence
    (`/Game/ThirdPerson/Blueprints/BP_PlayerCharacter_May.CharacterBrightnessNLightColor` (stale `/Game/Blueprints/Actors/LightToSwitch/CQBLevel1Light/BPI_SwitchInteract.SwitchInteract` _array_element))
    (`KismetMaterialLibrary.SetScalarParameterValue` "/Game/Characters/VTGCharacterShader/Player_LightColor.Player_LightColor" "NPRBrightnessOverall" 5.7)
    (`KismetMaterialLibrary.SetVectorParameterValue` "/Game/Characters/VTGCharacterShader/Player_LightColor.Player_LightColor" "NPRColorBlend" (`self.NPRColor_LightBasement`))))

(fn `UserConstructionScript`)