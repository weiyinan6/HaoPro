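; Interactable light switch for the CQB1 upper floor that toggles its spotlights between bright and dark, starting bright.
; IA_Interact plays the switch animation, then after a short delay sets every upper-floor spotlight's intensity.
; It also flips the lamp material through MPC_CQBLamp and updates NPR brightness and color in the Player_LightColor collection and on May's character, so character shading follows the room lighting.
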(event `self.ReceiveBeginPlay`
  ;[1 1 1] Set Bright at beginning
  (set `self.IsLightBright?` true))

(event `EnhancedInput|/Game/ThirdPerson/Input/Actions/IA_Interact`
  (params (ActionValue :type Boolean) (ElapsedSeconds :type "Float (double-precision)") (TriggeredSeconds :type "Float (double-precision)") (InputAction :type "InputAction Object Reference" :default "/Game/ThirdPerson/Input/Actions/IA_Interact.IA_Interact"))
  ;[1 1 1] Switch triggered Light Intensity Change
  (:`Triggered`
    (`self.SwitchInteract`)))

(event `self.SwitchInteract`
  (bind _cqb1lightswitch (`self.CQB1LightSwitch`))
  (bind _nprcolor (`self.NPRColor`))
  ;[1 1 1] Switch triggered Light Intensity Change
  (bind _outactors (`GameplayStatics.GetAllActorsOfClass` "/Game/ThirdPerson/Blueprints/BP_PlayerCharacter_May.BP_PlayerCharacter_May_C"))
  (for _array_element _outactors
    (if (`self.IsLightBright?`)
      (set `self.IsLightBright?` false)
      (`KismetSystemLibrary.PrintString` "TurnOffLight")
      ;;[1 1 1] Switch Anm
      (`SkeletalMeshComponent.PlayAnimation` _cqb1lightswitch "/Game/Blueprints/Actors/LightToSwitch/CQBLevel1Light/Anm/ANM_CQB1LightSwitch_LightOnToOff.ANM_CQB1LightSwitch_LightOnToOff" false)
      (`KismetSystemLibrary.Delay` 0.4)
      (bind _outactors_2 (`GameplayStatics.GetAllActorsOfClass` "/Game/Blueprints/Actors/LightToSwitch/CQBLevel1Light/BP_Light_CQB1_Spotlight_UpperFloor.BP_Light_CQB1_Spotlight_UpperFloor_C"))
      (for _array_element_2 _outactors_2
        (`LightComponent.SetIntensity` (`/Game/Blueprints/Actors/LightToSwitch/CQBLevel1Light/BP_LightToSwitch_SpotLight.SpotLight` _array_element_2) (`self.Dark Light Intensity_Switch`))
        ;[1 1 1] Light Material
        (`KismetMaterialLibrary.SetScalarParameterValue` "/Game/Blueprints/Actors/LightToSwitch/CQBLevel1Light/MPC_CQBLamp.MPC_CQBLamp" "TexTransition(Bright0 to Dark1)" 1.0)
        ;[0.001042 0.001042 0.001042] NPR Influence
        (`/Game/ThirdPerson/Blueprints/BP_PlayerCharacter_May.CharacterBrightnessNLightColor` _array_element)
        (`KismetMaterialLibrary.SetScalarParameterValue` "/Game/Characters/VTGCharacterShader/Player_LightColor.Player_LightColor" "NPRBrightnessOverall" 0.5)
        (`KismetMaterialLibrary.SetVectorParameterValue` "/Game/Characters/VTGCharacterShader/Player_LightColor.Player_LightColor" "NPRColorBlend" _nprcolor)
        ;[1 1 1] Set Character Variable
        (set `/Game/ThirdPerson/Blueprints/BP_PlayerCharacter_May.NPRBrightness_CCurrent` 0.5 _array_element))
      (else
        (set `self.IsLightBright?` true)
        (`KismetSystemLibrary.PrintString` "TurnOnLight")
        (`SkeletalMeshComponent.PlayAnimation` _cqb1lightswitch "/Game/Blueprints/Actors/LightToSwitch/CQBLevel1Light/Anm/ANM_CQB1LightSwitch_LightOffToOn.ANM_CQB1LightSwitch_LightOffToOn" false)
        (`KismetSystemLibrary.Delay` 0.2)
        (bind _outactors_3 (`GameplayStatics.GetAllActorsOfClass` "/Game/Blueprints/Actors/LightToSwitch/CQBLevel1Light/BP_Light_CQB1_Spotlight_UpperFloor.BP_Light_CQB1_Spotlight_UpperFloor_C"))
        (for _array_element_3 _outactors_3
          (`LightComponent.SetIntensity` (`/Game/Blueprints/Actors/LightToSwitch/CQBLevel1Light/BP_LightToSwitch_SpotLight.SpotLight` _array_element_3) (`self.Bright Light Intensity_Switch`))
          (`KismetMaterialLibrary.SetScalarParameterValue` "/Game/Blueprints/Actors/LightToSwitch/CQBLevel1Light/MPC_CQBLamp.MPC_CQBLamp" "TexTransition(Bright0 to Dark1)")
          (`/Game/ThirdPerson/Blueprints/BP_PlayerCharacter_May.CharacterBrightnessNLightColor` _array_element)
          (`KismetMaterialLibrary.SetScalarParameterValue` "/Game/Characters/VTGCharacterShader/Player_LightColor.Player_LightColor" "NPRBrightnessOverall" 5.5)
          (`KismetMaterialLibrary.SetVectorParameterValue` "/Game/Characters/VTGCharacterShader/Player_LightColor.Player_LightColor" "NPRColorBlend" _nprcolor)
          (set `/Game/ThirdPerson/Blueprints/BP_PlayerCharacter_May.NPRBrightness_CCurrent` 5.5 _array_element))))))

(fn `UserConstructionScript`)