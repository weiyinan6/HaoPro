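; Light switch for the CQB1 basement that toggles its spotlights between bright and dark on the Interact input.
; SwitchInteract flips IsLightBright, which starts true when a May player character exists, then sets the intensity of every BP_Light_CQB1_Spotlight_Basement.
; It also calls May's CharacterBrightnessNLightColor and writes brightness and color to the Player_LightColor parameter collection, matching NPR shading to the light state.
; The input event calls the toggle directly, with no proximity check.
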(event `EnhancedInput|/Game/ThirdPerson/Input/Actions/IA_Interact`
  (params (ActionValue :type Boolean) (ElapsedSeconds :type "Float (double-precision)") (TriggeredSeconds :type "Float (double-precision)") (InputAction :type "InputAction Object Reference" :default "/Game/ThirdPerson/Input/Actions/IA_Interact.IA_Interact"))
  (:`Triggered`
    (`self.SwitchInteract`)))

(event `self.ReceiveBeginPlay`
  ;[1 1 1] Set Bright at beginning
  (bind _outactors (`GameplayStatics.GetAllActorsOfClass` "/Game/ThirdPerson/Blueprints/BP_PlayerCharacter_May.BP_PlayerCharacter_May_C"))
  (for _ _outactors
    (set `self.IsLightBright?` true)))

(event `/Game/Blueprints/Actors/LightToSwitch/BPI_SwitchInteract.SwitchInteract`
  (bind _nprcolor_lightbasement (`self.NPRColor_LightBasement`))
  (bind _outactors (`GameplayStatics.GetAllActorsOfClass` "/Game/ThirdPerson/Blueprints/BP_PlayerCharacter_May.BP_PlayerCharacter_May_C"))
  (for _array_element _outactors
    ;[1 1 1] Switch triggered Light Intensity Change
    (if (`self.IsLightBright?`)
      (set `self.IsLightBright?` false)
      (`KismetSystemLibrary.PrintString` "TurnOffLight")
      (bind _outactors_2 (`GameplayStatics.GetAllActorsOfClass` "/Game/Blueprints/Actors/LightToSwitch/BP_Light_CQB1_Spotlight_Basement.BP_Light_CQB1_Spotlight_Basement_C"))
      (for _array_element_2 _outactors_2
        (`LightComponent.SetIntensity` (`/Game/Blueprints/Actors/LightToSwitch/BP_LightToSwitch_SpotLight.SpotLight` _array_element_2) (`self.Dark Light Intensity_Switch`))
        ;[0.001042 0.001042 0.001042] NPR Influence
        (`/Game/ThirdPerson/Blueprints/BP_PlayerCharacter_May.CharacterBrightnessNLightColor` _array_element)
        (`KismetMaterialLibrary.SetScalarParameterValue` "/Game/Characters/VTGCharacterShader/Player_LightColor.Player_LightColor" "NPRBrightnessOverall" 0.6)
        (`KismetMaterialLibrary.SetVectorParameterValue` "/Game/Characters/VTGCharacterShader/Player_LightColor.Player_LightColor" "NPRColorBlend" _nprcolor_lightbasement))
      (else
        (set `self.IsLightBright?` true)
        (`KismetSystemLibrary.PrintString` "TurnOnLight")
        (bind _outactors_3 (`GameplayStatics.GetAllActorsOfClass` "/Game/Blueprints/Actors/LightToSwitch/BP_Light_CQB1_Spotlight_Basement.BP_Light_CQB1_Spotlight_Basement_C"))
        (for _array_element_3 _outactors_3
          (`LightComponent.SetIntensity` (`/Game/Blueprints/Actors/LightToSwitch/BP_LightToSwitch_SpotLight.SpotLight` _array_element_3) (`self.Bright Light Intensity_Switch`))
          (`/Game/ThirdPerson/Blueprints/BP_PlayerCharacter_May.CharacterBrightnessNLightColor` _array_element)
          (`KismetMaterialLibrary.SetScalarParameterValue` "/Game/Characters/VTGCharacterShader/Player_LightColor.Player_LightColor" "NPRBrightnessOverall" 5.7)
          (`KismetMaterialLibrary.SetVectorParameterValue` "/Game/Characters/VTGCharacterShader/Player_LightColor.Player_LightColor" "NPRColorBlend" _nprcolor_lightbasement))))))

(fn `UserConstructionScript`)