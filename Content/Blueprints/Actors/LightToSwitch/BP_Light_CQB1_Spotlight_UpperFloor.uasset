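; BP_Light_CQB1_Spotlight_UpperFloor is a switchable spotlight actor, named for the upper floor of CQB1.
; Its LightIntensity event is empty, with a note that the switch Blueprint already does the same work.
; Disconnected leftover nodes would flip IsLightBright and set the SpotLight between local and dark intensity with a debug print, but they never run.
; The construction script only calls its parent.
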(event `self.Light Intensity`
  (params (LightIntensity :type "/Game/Blueprints/Actors/LightToSwitch/BP_Light_CQB1_Spotlight_Basement Object Reference"))
  ;[1 1 1] Same with Switch BP, no need to do it again
)

(fn `UserConstructionScript`
  (`parent.UserConstructionScript`))