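; Actor component that owns a radial wheel menu and exposes an API to show, hide, query and edit its slots.
; On BeginPlay it polls for a valid player state, skipping dedicated servers, then creates the collapsed wheel widget with itself as reference.
; Item edits refresh the widget, adding or removing slots regenerates it, and active-slot setters only update the data.
; Selection and active-slot changes are re-broadcast through event dispatchers.
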(event `self.ReceiveBeginPlay`
  ;[0 0 0] Create the Radial Wheel Widget
  (`self.Wait For Player State`)
  (bind _returnvalue (`|CreateWidget` "/Game/Procedural_Radial_Wheel_Menu/Blueprints/Radial_Wheel_WB.Radial_Wheel_WB_C" null self))
  (bind _output_get (set `self.Radial Wheel Widget` _returnvalue))
  (`UserWidget.AddToViewport` _output_get (`self.Viewport Z Order`))
  (`Widget.SetVisibility` _output_get "Collapsed"))

(event `Show Radial Wheel`
  ;[0 0 0] Show Radial Wheel
  (`/Game/Procedural_Radial_Wheel_Menu/Blueprints/Radial_Wheel_WB.Show Radial Wheel` (`self.Radial Wheel Widget`)))

(event `Hide Radial Wheel`
  ;[0 0 0] Hide Radial Wheel
  (`/Game/Procedural_Radial_Wheel_Menu/Blueprints/Radial_Wheel_WB.Hide Radial Wheel` (`self.Radial Wheel Widget`)))

(event `Selected Slot Changed`
  (params (`Selected Slot` :type "/Game/Procedural_Radial_Wheel_Menu/Blueprints/Structs/Radial_Wheel_Slot_Struct Structure") (`Valid?` :type Boolean))
  ;[0 0 0] On Radial Wheel Selection Changed
  (`self.On Selection Changed` `Selected Slot` `Valid?`))

(event `Active Slot Changed`
  (params (`Active Slot` :type "/Game/Procedural_Radial_Wheel_Menu/Blueprints/Structs/Radial_Wheel_Slot_Struct Structure"))
  ;[0 0 0] On Radial Wheel Selection Changed
  (`self.On Active Slot Changed` `Active Slot`))

(fn `Add Slot`
  (params (Slot :type "/Game/Procedural_Radial_Wheel_Menu/Blueprints/Structs/Radial_Wheel_Slot_Struct Structure"))
  ;[0 0 0] Adds a slot at the end of the slots array.
  (`KismetArrayLibrary.Array_Add` (`self.Slots`) Slot)
  (`/Game/Procedural_Radial_Wheel_Menu/Blueprints/Radial_Wheel_WB.Generate Radial Wheel` (`self.Radial Wheel Widget`) (`self.Slots`)))

(fn `Clear Active Slots`
  ;[0 0 0] Deactivates all active slots.
  (bind _slot (`self.For Each Slot`)
    (:`LoopBody`
      (setmembers `/Game/Procedural_Radial_Wheel_Menu/Blueprints/Structs/Radial_Wheel_Slot_Struct` :`StructRef` _slot :`Is Active?` false))))

(fn `Get Current Active Slot`
  (returns (`Valid?` :type Boolean) (ReturnValue :type "/Game/Procedural_Radial_Wheel_Menu/Blueprints/Structs/Radial_Wheel_Slot_Struct Structure"))
  ;[0 0 0] Gets the currently active slot.
  (bind _slot (`self.For Each Slot`)
    (:`LoopBody`
      (if (`.IsActive?_17_EF171DDB475CE5E95715EDA0D8D4DAC7` (break `/Game/Procedural_Radial_Wheel_Menu/Blueprints/Structs/Radial_Wheel_Slot_Struct` _slot))
        (return true _slot)))
    (:`Completed`
      (return false))))

(fn `Get Current Selected Slot`
  (returns (`Valid?` :type Boolean) (ReturnValue :type "/Game/Procedural_Radial_Wheel_Menu/Blueprints/Structs/Radial_Wheel_Slot_Struct Structure"))
  ;[0 0 0] Gets the currently selected slot, only works if the wheel is open.
  (if (`self.Is Wheel Open?`)
    (bind _current_slot (`/Game/Procedural_Radial_Wheel_Menu/Blueprints/Radial_Wheel_WB.Current Slot` (`self.Radial Wheel Widget`))
      (:`then`
        (return true (`/Game/Procedural_Radial_Wheel_Menu/Blueprints/Radial_Wheel_Item_WB.Slot Data` _current_slot)))
      (:`else`
        _)))
  (return false))

(fn `Insert Slot`
  (params (`Slot Index` :type Integer) (Slot :type "/Game/Procedural_Radial_Wheel_Menu/Blueprints/Structs/Radial_Wheel_Slot_Struct Structure"))
  ;[0 0 0] Adds a slot at the specified index of the slots array.
  (`KismetArrayLibrary.Array_Insert` (`self.Slots`) Slot (`KismetMathLibrary.Clamp` `Slot Index` 0 (+ (`KismetArrayLibrary.Array_LastIndex` (`self.Slots`)) 1)))
  (`/Game/Procedural_Radial_Wheel_Menu/Blueprints/Radial_Wheel_WB.Generate Radial Wheel` (`self.Radial Wheel Widget`) (`self.Slots`)))

(fn `Is Wheel Open?`
  (returns (ReturnValue :type Boolean))
  ;[0 0 0] Returns whether or not the wheel is open.
  (return (`/Game/Procedural_Radial_Wheel_Menu/Blueprints/Radial_Wheel_WB.Wheel Opened?` (`self.Radial Wheel Widget`))))

(fn `Remove Item On Slot`
  (params (`Slot Index` :type Integer))
  (returns (`Successful?` :type Boolean))
  (bind _slots (`self.Slots`))
  ;[0 0 0] Removes the item on the slot at the specified index (if it exists).
  (if (`KismetArrayLibrary.Array_IsValidIndex` _slots `Slot Index`)
    (setmembers `/Game/Procedural_Radial_Wheel_Menu/Blueprints/Structs/Radial_Wheel_Slot_Struct` :`StructRef` (`|GetArrayItem` _slots `Slot Index`) :`Has Item?` false :`Item` (struct :`IconSize` (32.0 32.0) :`IconTransform` (struct :`Translation` (0.0 0.0) :`Scale` (1.0 1.0) :`Shear` (0.0 0.0)) :`InfoTextTransform` (struct :`Translation` (0.0 50.0) :`Scale` (1.0 1.0) :`Shear` (0.0 0.0))))
    (`/Game/Procedural_Radial_Wheel_Menu/Blueprints/Radial_Wheel_WB.Refresh Radial Wheel Slots` (`self.Radial Wheel Widget`))
    (return true)
    (else
      (return false))))

(fn `Remove Slot`
  (params (`Slot Index` :type Integer))
  (returns (`Successful?` :type Boolean))
  ;[0 0 0] Removes the slot at the specified index (if it exists).
  (if (`KismetArrayLibrary.Array_IsValidIndex` (`self.Slots`) `Slot Index`)
    (`KismetArrayLibrary.Array_Remove` (`self.Slots`) `Slot Index`)
    (`/Game/Procedural_Radial_Wheel_Menu/Blueprints/Radial_Wheel_WB.Generate Radial Wheel` (`self.Radial Wheel Widget`) (`self.Slots`))
    (return true)
    (else
      (return false))))

(fn `Set Item On Slot`
  (params (`Slot Index` :type Integer) (Item :type "/Game/Procedural_Radial_Wheel_Menu/Blueprints/Structs/Radial_Wheel_Item_Struct Structure"))
  (returns (`Successful?` :type Boolean))
  (bind _slots (`self.Slots`))
  ;[0 0 0] Sets the item on the slot at the specified slot index (if it exists).
  (if (`KismetArrayLibrary.Array_IsValidIndex` _slots `Slot Index`)
    (setmembers `/Game/Procedural_Radial_Wheel_Menu/Blueprints/Structs/Radial_Wheel_Slot_Struct` :`StructRef` (`|GetArrayItem` _slots `Slot Index`) :`Has Item?` true :`Item` (`local.Item`))
    (`/Game/Procedural_Radial_Wheel_Menu/Blueprints/Radial_Wheel_WB.Refresh Radial Wheel Slots` (`self.Radial Wheel Widget`))
    (return true)
    (else
      (return false))))

(fn `Set Slot Active`
  (params (`Slot Index` :type Integer))
  (returns (`Successful?` :type Boolean))
  ;[0 0 0] Sets the slot at the specified index as active and deactivates all other slots (if it exists).
  (if (`KismetArrayLibrary.Array_IsValidIndex` (`self.Slots`) `Slot Index`)
    (bind (_slot _index) (`self.For Each Slot`)
      (:`LoopBody`
        (setmembers `/Game/Procedural_Radial_Wheel_Menu/Blueprints/Structs/Radial_Wheel_Slot_Struct` :`StructRef` _slot :`Is Active?` (== _index (`local.Slot Index`))))
      (:`Completed`
        (return true)))
    (else
      (return false))))