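; Inventory component that lets the player pick up items and drop them back into the world.
; On Interact, a sphere trace from the follow camera finds pickup actors, stores their data and destroys them.
; Items live in a map keyed by name, so duplicates stack by amount.
; Removing one decrements or deletes the entry, then spawns the item ahead of the connected actor, using a downward trace to find the surface.
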(event `EnhancedInput|/Game/ThirdPerson/Input/Actions/IA_Interact`
  (params (ActionValue :type Boolean) (ElapsedSeconds :type "Float (double-precision)") (TriggeredSeconds :type "Float (double-precision)") (InputAction :type "InputAction Object Reference" :default "/Game/ThirdPerson/Input/Actions/IA_Interact.IA_Interact"))
  (:`Completed`
    (bind _asbp_player_character_1 (cast `/Game/ThirdPerson/Blueprints/BP_PlayerCharacter1` (`GameplayStatics.GetPlayerCharacter` 0)))
    (bind _followcamera (`/Game/ThirdPerson/Blueprints/BP_PlayerCharacter1.FollowCamera` _asbp_player_character_1))
    (bind _returnvalue (`SceneComponent.K2_GetComponentLocation` _followcamera))
    (bind _outhit (`KismetSystemLibrary.SphereTraceSingle` :`Start` _returnvalue :`End` (+ _returnvalue (* (`SceneComponent.GetForwardVector` _followcamera) 5000.0)) :`Radius` 30.0 :`TraceChannel` "TraceTypeQuery1" :`DrawDebugType` "ForDuration"))
    (if true
      (bind (_bblockinghit _binitialoverlap _time _distance _location _impactpoint _normal _impactnormal _physmat _hitactor) (`GameplayStatics.BreakHitResult` _outhit))
      (bind _added_ (`self.Try AddItem` _hitactor))
      (if _added_
        (`Actor.K2_DestroyActor` _hitactor)))))

(fn `AddItemToInventory`
  (params (Item :type "/Game/Inventory/S_ItemData Structure"))
  (`BlueprintMapLibrary.Map_Add` (`self.Inventory`) (`.Name_2_D6255EF143A0A4E3F058A19AE633ED11` (break `/Game/Inventory/S_ItemData` Item)) Item))

(fn `IncreaseItemAmount`
  (params (Item :type "/Game/Inventory/S_ItemData Structure"))
  (locals (ItemName :type String))
  (bind _value (`BlueprintMapLibrary.Map_Find` (`self.Inventory`) (`local.ItemName`)))
  (set `local.ItemName` (`.Name_2_D6255EF143A0A4E3F058A19AE633ED11` (break `/Game/Inventory/S_ItemData` Item)))
  (bind _result (`/Engine/EditorBlueprintResources/StandardMacros.IncrementInt` (`.Amount_12_FFBBFAB04036CA0A35BD85866146C324` (break `/Game/Inventory/S_ItemData` _value)))
    (:`  `
      (bind _structout (setmembers `/Game/Inventory/S_ItemData` :`StructRef` _value :`Amount` _result))
      (`BlueprintMapLibrary.Map_Add` (`self.Inventory`) (`local.ItemName`) _structout))))

(fn `IsItemAlreadyInInventory?`
  (params (Item :type "/Game/Inventory/S_ItemData Structure"))
  (returns (ReturnValue :type Boolean))
  (return (`BlueprintMapLibrary.Map_Contains` (`self.Inventory`) (`.Name_2_D6255EF143A0A4E3F058A19AE633ED11` (break `/Game/Inventory/S_ItemData` Item)))))

(fn `Remove Single Item`
  (params (Key :type "String (by ref)"))
  (returns (ItemFullyRemoved :type Boolean) (NewItemData :type "/Game/Inventory/S_ItemData Structure"))
  (bind (_value _returnvalue) (`BlueprintMapLibrary.Map_Find` (`self.Inventory`) Key))
  (bind (_name _category _description _amount) (break `/Game/Inventory/S_ItemData` _value))
  (if _returnvalue
    (if (> _amount 1)
      (bind _structout (setmembers `/Game/Inventory/S_ItemData` :`StructRef` _value :`Amount` (- _amount 1)))
      (`BlueprintMapLibrary.Map_Add` (`self.Inventory`) (`local.Key`) _structout)
      (bind _impactpoint (`self.TraceFromAbove`))
      (`self.SpawnItem` (`.ItemClass_16_48B6BB50434AFC3A81E22DA4DBC18DB0` (break `/Game/Inventory/S_ItemData` _structout)) _impactpoint)
      (return false _structout)
      (else
        (bind _output_get (set `self.DeletedItem` _value))
        (`BlueprintMapLibrary.Map_Remove` (`self.Inventory`) (`local.Key`))
        (bind _impactpoint_2 (`self.TraceFromAbove`))
        (`self.SpawnItem` (`.ItemClass_16_48B6BB50434AFC3A81E22DA4DBC18DB0` (break `/Game/Inventory/S_ItemData` _output_get)) _impactpoint_2)
        (return true)))))

(fn `SpawnItem`
  (params (Class :type "Actor Class Reference") (Position :type "Vector Structure"))
  (`|SpawnActorFromClass` Class (`KismetMathLibrary.MakeTransform` (+ Position (0.0 0.0 50.0))) "Undefined" "MultiplyWithRoot" null null))

(fn `TraceFromAbove`
  (returns (ImpactPoint :type "Vector Structure"))
  (bind _connectedactor (`self.ConnectedActor`))
  (bind _returnvalue (`SceneComponent.K2_GetComponentLocation` (`Character.Mesh` _connectedactor)))
  (bind _x (.x (* (`SceneComponent.GetForwardVector` (`/Game/ThirdPerson/Blueprints/BP_PlayerCharacter1.FollowCamera` _connectedactor)) 200.0)))
  (bind _y (.y (* (`SceneComponent.GetForwardVector` (`/Game/ThirdPerson/Blueprints/BP_PlayerCharacter1.FollowCamera` _connectedactor)) 200.0)))
  (bind (_outhit _returnvalue_2) (`KismetSystemLibrary.SphereTraceSingle` :`Start` (+ _returnvalue (`KismetMathLibrary.MakeVector` _x _y 2000.0)) :`End` (+ _returnvalue (`KismetMathLibrary.MakeVector` _x _y -1000.0)) :`Radius` 5.0 :`TraceChannel` "TraceTypeQuery1" :`DrawDebugType` "ForDuration"))
  (if _returnvalue_2
    (bind (_bblockinghit _binitialoverlap _time _distance _location _impactpoint _normal _impactnormal _physmat _hitactor _hitcomponent _hitbonename _bonename _hititem _elementindex _faceindex _tracestart _traceend) (`GameplayStatics.BreakHitResult` _outhit))
    (return _impactpoint)
    (else
      (return _traceend))))

(fn `Try AddItem`
  (params (HitActor :type "Actor Object Reference"))
  (returns (`Added?` :type Boolean))
  (locals (CurrentItem :type "/Game/Inventory/S_ItemData Structure"))
  (bind _currentitem (`local.CurrentItem`))
  (bind _asa_master_pick_up_item (cast `/Game/Inventory/A_MasterPickUpItem` HitActor)
    (:`then`
      (bind _output_get (set `local.CurrentItem` (`/Game/Inventory/A_MasterPickUpItem.GetItemData` _asa_master_pick_up_item)))
      (if (`self.IsItemAlreadyInInventory?` _output_get)
        (`self.IncreaseItemAmount` _currentitem)
        (else
          (`self.AddItemToInventory` _currentitem)))
      (`KismetSystemLibrary.PrintString` (`KismetStringLibrary.Concat_StrStr` (`.Name_2_D6255EF143A0A4E3F058A19AE633ED11` (break `/Game/Inventory/S_ItemData` _currentitem)) "Added"))
      (return true))
    (:`CastFailed`
      (set `local.CurrentItem` (struct))
      (return false))))