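; Player inventory component that stores picked-up items in a name-keyed map of stackable item structs.
; On interact, a camera sphere trace finds pickup actors, adds or increments their entry, posts an info message and destroys them.
; Removing an item spawns its class back into the world at a traced point, while using one just decrements it.
; Name switches apply item effects: ammo on pickup, healing on use.
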(event `EnhancedInput|/Game/ThirdPerson/Input/Actions/IA_Interact`
  (params (ActionValue :type Boolean) (ElapsedSeconds :type "Float (double-precision)") (TriggeredSeconds :type "Float (double-precision)") (InputAction :type "InputAction Object Reference" :default "/Game/ThirdPerson/Input/Actions/IA_Interact.IA_Interact"))
  (:`Completed`
    (bind _asbp_player_character_may (cast `/Game/ThirdPerson/Blueprints/BP_PlayerCharacter_May` (`GameplayStatics.GetPlayerCharacter` 0)))
    (bind _followcamera (`/Game/ThirdPerson/Blueprints/BP_PlayerCharacter_May.FollowCamera` _asbp_player_character_may))
    (bind _returnvalue (`SceneComponent.K2_GetComponentLocation` _followcamera))
    (bind (_outhit _returnvalue_2) (`KismetSystemLibrary.SphereTraceSingle` _returnvalue (+ _returnvalue (* (`SceneComponent.GetForwardVector` _followcamera) 400.0)) 5.0 "TraceTypeQuery1"))
    (if _returnvalue_2
      (bind (_bblockinghit _binitialoverlap _time _distance _location _impactpoint _normal _impactnormal _physmat _hitactor) (`GameplayStatics.BreakHitResult` _outhit))
      (bind _added_ (`self.Try AddItem` _hitactor))
      (if _added_
        (`Actor.K2_DestroyActor` _hitactor)))))

(fn `AddItemToInventory`
  (params (Item :type "/Game/Inventory/Inventory_CQB/S_InventoryItemData Structure"))
  (`BlueprintMapLibrary.Map_Add` (`self.Inventory`) (`.Name_2_D6255EF143A0A4E3F058A19AE633ED11` (break `/Game/Inventory/Inventory_CQB/S_InventoryItemData` Item)) Item))

(fn `IncreaseItemAmount`
  (params (Item :type "/Game/Inventory/Inventory_CQB/S_InventoryItemData Structure"))
  (returns (ItemOut :type "/Game/Inventory/Inventory_CQB/S_InventoryItemData Structure (by ref)"))
  (locals (ItemName :type String))
  (bind _value (`BlueprintMapLibrary.Map_Find` (`self.Inventory`) (`local.ItemName`)))
  (set `local.ItemName` (`.Name_2_D6255EF143A0A4E3F058A19AE633ED11` (break `/Game/Inventory/Inventory_CQB/S_InventoryItemData` Item)))
  (bind _result (`/Engine/EditorBlueprintResources/StandardMacros.IncrementInt` (`.Amount_12_FFBBFAB04036CA0A35BD85866146C324` (break `/Game/Inventory/Inventory_CQB/S_InventoryItemData` _value)))
    (:`  `
      (bind _structout (setmembers `/Game/Inventory/Inventory_CQB/S_InventoryItemData` :`StructRef` _value :`Amount` _result))
      (`BlueprintMapLibrary.Map_Add` (`self.Inventory`) (`local.ItemName`) _structout)
      (return _structout))))

(fn `IsItemAlreadyInInventory?`
  (params (Item :type "/Game/Inventory/Inventory_CQB/S_InventoryItemData Structure"))
  (returns (ReturnValue :type Boolean))
  (return (`BlueprintMapLibrary.Map_Contains` (`self.Inventory`) (`.Name_2_D6255EF143A0A4E3F058A19AE633ED11` (break `/Game/Inventory/Inventory_CQB/S_InventoryItemData` Item)))))

(fn `ItemPickUpFunction`
  (params (ItemName :type Name))
  (bind _connectedactor (`self.ConnectedActor`))
  ;[1 1 1] 在这里填上物品名称，后面加对应的功能
  (switch `name` ItemName
    (:`Ammo Charge`
      (set `/Game/ThirdPerson/Blueprints/BP_PlayerCharacter_May.LeftAmmo` (+ (`/Game/ThirdPerson/Blueprints/BP_PlayerCharacter_May.LeftAmmo` _connectedactor) 4) _connectedactor))))

(fn `ItemUsedFunction`
  (params (ItemName :type Name))
  (switch `name` ItemName
    (:`Recovery Injection`
      (bind _asbp_player_character_may (cast `/Game/ThirdPerson/Blueprints/BP_PlayerCharacter_May` (`GameplayStatics.GetPlayerCharacter` 0)))
      (`/Game/ThirdPerson/Blueprints/BP_PlayerCharacter_May.UpdateHealth` _asbp_player_character_may 50))))

(fn `Remove Single Item`
  (params (Key :type "String (by ref)"))
  (returns (ItemFullyRemoved :type Boolean) (NewItemData :type "/Game/Inventory/Inventory_CQB/S_InventoryItemData Structure"))
  (bind (_value _returnvalue) (`BlueprintMapLibrary.Map_Find` (`self.Inventory`) Key))
  (bind (_name _category _description _amount) (break `/Game/Inventory/Inventory_CQB/S_InventoryItemData` _value))
  (if _returnvalue
    (if (> _amount 1)
      (bind _structout (setmembers `/Game/Inventory/Inventory_CQB/S_InventoryItemData` :`StructRef` _value :`Amount` (- _amount 1)))
      (`BlueprintMapLibrary.Map_Add` (`self.Inventory`) (`local.Key`) _structout)
      (bind _impactpoint (`self.TraceFromAbove`))
      (`self.SpawnItem` (`.ItemClass_16_48B6BB50434AFC3A81E22DA4DBC18DB0` (break `/Game/Inventory/Inventory_CQB/S_InventoryItemData` _structout)) _impactpoint)
      (return false _structout)
      (else
        (bind _output_get (set `self.DeletedItem` _value))
        (`BlueprintMapLibrary.Map_Remove` (`self.Inventory`) (`local.Key`))
        (bind _impactpoint_2 (`self.TraceFromAbove`))
        (`self.SpawnItem` (`.ItemClass_16_48B6BB50434AFC3A81E22DA4DBC18DB0` (break `/Game/Inventory/Inventory_CQB/S_InventoryItemData` _output_get)) _impactpoint_2)
        (return true)))))

(fn `SpawnItem`
  (params (Class :type "Actor Class Reference") (Position :type "Vector Structure"))
  (`|SpawnActorFromClass` Class (`KismetMathLibrary.MakeTransform` (+ Position (0.0 0.0 50.0))) "Undefined" "MultiplyWithRoot" null null))

(fn `TraceFromAbove`
  (returns (ImpactPoint :type "Vector Structure"))
  (bind _connectedactor (`self.ConnectedActor`))
  (bind _followcamera (`/Game/ThirdPerson/Blueprints/BP_PlayerCharacter_May.FollowCamera` _connectedactor))
  (bind (_outhit _returnvalue) (`KismetSystemLibrary.SphereTraceSingle` :`Start` (`Actor.GetActorEyesViewPoint` _connectedactor) :`End` (+ (`SceneComponent.K2_GetComponentLocation` _followcamera) (* (`SceneComponent.GetForwardVector` _followcamera) 400.0)) :`Radius` 5.0 :`TraceChannel` "TraceTypeQuery1" :`DrawDebugType` "ForDuration"))
  (if _returnvalue
    (bind (_bblockinghit _binitialoverlap _time _distance _location _impactpoint _normal _impactnormal _physmat _hitactor _hitcomponent _hitbonename _bonename _hititem _elementindex _faceindex _tracestart _traceend) (`GameplayStatics.BreakHitResult` _outhit))
    (return _impactpoint)
    (else
      (return _traceend))))

(fn `Try AddItem`
  (params (HitActor :type "Actor Object Reference"))
  (returns (`Added?` :type Boolean))
  (locals (CurrentItem :type "/Game/Inventory/Inventory_CQB/S_InventoryItemData Structure"))
  (bind _wbinfoscreenref (`self.WbInfoScreenRef`))
  (bind _currentitem (`local.CurrentItem`))
  (bind (_name _category _description _amount) (break `/Game/Inventory/Inventory_CQB/S_InventoryItemData` _currentitem))
  (bind _asa_master_pick_up_item (cast `/Game/Inventory/Inventory_CQB/A_MasterPickUpItem` HitActor)
    (:`then`
      (cast `/Game/ThirdPerson/Blueprints/BP_PlayerCharacter_May` HitActor
        (:`then`
          _)
        (:`CastFailed`
          _))
      (bind _output_get (set `local.CurrentItem` (`/Game/Inventory/Inventory_CQB/A_MasterPickUpItem.GetInventoryItemData` _asa_master_pick_up_item)))
      (if (`self.IsItemAlreadyInInventory?` _output_get)
        (bind _itemout (`self.IncreaseItemAmount` _currentitem))
        (bind (_name_2 _category_2 _description_2 _amount_2) (break `/Game/Inventory/Inventory_CQB/S_InventoryItemData` _itemout))
        (message `/Game/Blueprints/Interface/BPI_ItemInfoSystem.CreateInfoItem` _wbinfoscreenref (`KismetStringLibrary.Concat_StrStr` _name_2 "  Added   " "(" (`KismetStringLibrary.Conv_IntToString` _amount_2) ")"))
        (else
          (`self.AddItemToInventory` _currentitem)
          (message `/Game/Blueprints/Interface/BPI_ItemInfoSystem.CreateInfoItem` _wbinfoscreenref (`KismetStringLibrary.Concat_StrStr` _name "" "Added"))))
      (`self.ItemPickUpFunction` (`KismetStringLibrary.Conv_StringToName` _name))
      (return true))
    (:`CastFailed`
      (set `local.CurrentItem` (struct))
      (return false))))

(fn `UniqueFunction`
  (params (HasFunction :type Boolean) (HitActor :type "Actor Object Reference")))

(fn `UseHealthItem`
  (params (ItemName :type Name))
  (bind _outactors (`GameplayStatics.GetAllActorsOfClass` "/Game/ThirdPerson/Blueprints/BP_PlayerCharacter_May.BP_PlayerCharacter_May_C"))
  (for _array_element _outactors
    (switch `name` ItemName
      (:`Recovery Injection`
        (if (`.ReturnValue` (`BlueprintMapLibrary.Map_Find` (`self.Inventory`) "Recovery Injection"))
          (set `/Game/ThirdPerson/Blueprints/BP_PlayerCharacter_May.Health` (+ (`/Game/ThirdPerson/Blueprints/BP_PlayerCharacter_May.Health` _array_element) 50) _array_element)
          (else
            (`KismetSystemLibrary.PrintString` "No Selected Health Item")))))))

(fn `UseItem`
  (params (Key :type "String (by ref)"))
  (returns (ItemFullyRemoved :type Boolean) (NewItemData :type "/Game/Inventory/Inventory_CQB/S_InventoryItemData Structure"))
  (bind (_value _returnvalue) (`BlueprintMapLibrary.Map_Find` (`self.Inventory`) Key))
  (bind (_name _category _description _amount) (break `/Game/Inventory/Inventory_CQB/S_InventoryItemData` _value))
  (if _returnvalue
    (if (> _amount 1)
      (bind _structout (setmembers `/Game/Inventory/Inventory_CQB/S_InventoryItemData` :`StructRef` _value :`Amount` (- _amount 1)))
      (`self.ItemUsedFunction` (`KismetStringLibrary.Conv_StringToName` (`local.Key`)))
      (`BlueprintMapLibrary.Map_Add` (`self.Inventory`) (`local.Key`) _structout)
      (return false _structout)
      (else
        (set `self.DeletedItem` _value)
        (`BlueprintMapLibrary.Map_Remove` (`self.Inventory`) (`local.Key`))
        (`self.ItemUsedFunction` (`KismetStringLibrary.Conv_StringToName` (`local.Key`)))
        (return true)))))