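; SmokeBomb_BP is a stealth smoke bomb actor that temporarily notifies nearby characters' SuspicionComponents that they are inside smoke.
; On BeginPlay it spawns a Niagara burst, waits briefly, then takes a single snapshot of overlapping Characters, caching their SuspicionComponents and calling InSmokeBomb.
; After SmokeDuration it calls OutSmokeBomb on those still valid and destroys itself.
; Characters entering after the snapshot are not affected.
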(event `self.ReceiveBeginPlay`
  (`NiagaraFunctionLibrary.SpawnSystemAtLocation` "/Game/StealthSystem/Pickups/PoisonSeed_Explosion_NS.PoisonSeed_Explosion_NS" (`self.K2_GetActorLocation`))
  (`KismetSystemLibrary.Delay` 0.2)
  (for _array_element (`self.GetOverlappingActors` "/Script/Engine.Character")
    (bind _returnvalue (`self.GetComponentByClass` _array_element "/Game/StealthSystem/Enemy/Components/SuspicionComponent.SuspicionComponent_C"))
    (`/Engine/EditorBlueprintResources/StandardMacros.IsValid` _returnvalue
      (:`Is Valid`
        (`KismetArrayLibrary.Array_Add` (`self.AffectedComponents`) _returnvalue)
        (`/Game/StealthSystem/Enemy/Components/SuspicionComponent.InSmokeBomb` _returnvalue))))
  (`KismetSystemLibrary.Delay` (`self.SmokeDuration`))
  (for _array_element_2 (`self.AffectedComponents`)
    (`/Engine/EditorBlueprintResources/StandardMacros.IsValid` _array_element_2
      (:`Is Valid`
        (`/Game/StealthSystem/Enemy/Components/SuspicionComponent.OutSmokeBomb` _array_element_2))))
  (`self.K2_DestroyActor`))

(fn `UserConstructionScript`)