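; Male melee Soldier of Kaalor enemy AI character, with modular outfit meshes, health and scan highlighting.
; Combat changes from AIBehaviorsComponent move the weapon between sockets via server-to-multicast events.
; MeleeCollisionComponent traces weapon sockets and spawns hit effects.
; Point damage triggers directional hit reactions, or ragdoll when health equals exactly zero, while being scanned briefly shows a mark widget and custom-depth highlight.
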(event `self.AIBehaviorsComponent.OnInCombatChange`
  (params (IsInCombat :type Boolean))
  ;[1 0.6706 0.2488] On Combat change
  (`self.Server_SwitchWeapon` IsInCombat))

(event `Server_SwitchWeapon`
  (params (Equip :type Boolean))
  ;[1 0.6706 0.2488] Switch Weapon Socket
  (`self.Multicast_SwitchWeapon` Equip))

(event `Multicast_SwitchWeapon`
  (params (Equip :type Boolean))
  (bind _mesh (`self.Mesh`))
  (bind _weapon (`self.Weapon`))
  ;[1 0.6706 0.2488] Switch Weapon Socket
  (if Equip
    (`SceneComponent.K2_AttachToComponent` _weapon _mesh (`self.WeaponEquipSocket`) "SnapToTarget" "SnapToTarget" "SnapToTarget" true)
    (else
      (`SceneComponent.K2_AttachToComponent` _weapon _mesh (`self.WeaponUnequipSocket`) "SnapToTarget" "SnapToTarget" "SnapToTarget" true))))

(event `self.MeleeCollisionComponent.OnCollisionEnabled`
  (params (CollisionPart :type "/Game/AIBehaviorSystem/Blueprint/Enums/E_CollisionPart Enum" :default "NewEnumerator8"))
  (bind _weapon (`self.Weapon`))
  ;[1 0.6706 0.2488] On Collision Enabled
  (switch `/Game/AIBehaviorSystem/Blueprint/Enums/E_CollisionPart` CollisionPart
    (:`NewEnumerator0`
      (`/Game/AIBehaviorSystem/Blueprint/Component/BP_CollisionComponent.SetCollisions` (`self.MeleeCollisionComponent`) (`|MakeArray` (make `/Game/AIBehaviorSystem/Blueprint/Struct/F_CollisionComponent` _weapon (`SceneComponent.GetAllSocketNames` _weapon)))))))

(event `self.MeleeCollisionComponent.OnHit`
  (params (HitResult :type "HitResult Structure"))
  ;[1 0.6706 0.2488] On Collision Hit
  (`/Game/AIBehaviorSystem/Blueprint/Component/BP_CollisionComponent.Server_Spawn Hit VFX and Sound` (`self.MeleeCollisionComponent`) HitResult (`self.MeleeHitVFX`) (`self.MeleeHitSound`) (1.5 1.5 1.5)))

(event `self.ReceivePointDamage`
  (params (Damage :type "Float (single-precision)") (DamageType :type "DamageType Object Reference") (HitLocation :type "Vector Structure") (HitNormal :type "Vector Structure") (HitComponent :type "PrimitiveComponent Object Reference") (BoneName :type Name) (ShotFromDirection :type "Vector Structure") (InstigatedBy :type "Controller Object Reference") (DamageCauser :type "Actor Object Reference") (HitInfo :type "HitResult Structure (by ref)"))
  (bind _aibehaviorscomponent (`self.AIBehaviorsComponent`))
  (bind _direction (`/Game/AIBehaviorSystem/Blueprint/Library/BP_FunctionLibrary.GetHitDirection` ShotFromDirection self))
  ;[1 0.3824 0.3443] Recieve Damage
  (`KismetSystemLibrary.PrintString` (`KismetStringLibrary.Conv_DoubleToString` Damage))
  (bind _output_get (set `self.CurrentHealth` (- (`self.CurrentHealth`) Damage)))
  (if (== _output_get 0.0)
    (`/Game/AIBehaviorSystem/Blueprint/Component/BP_AIBehaviorsComponent.DeadRagdoll` _aibehaviorscomponent ShotFromDirection BoneName 1.0 _direction)
    (`ActorComponent.Deactivate` _aibehaviorscomponent)
    (else
      (`/Game/AIBehaviorSystem/Blueprint/Component/BP_AIBehaviorsComponent.Hitted` _aibehaviorscomponent _direction))))

(event `self.ReceiveAnyDamage`
  (params (Damage :type "Float (single-precision)") (DamageType :type "DamageType Object Reference") (InstigatedBy :type "Controller Object Reference") (DamageCauser :type "Actor Object Reference"))
  ;[1 1 1] ANYDMG
)

(event `/Game/AIBehaviorSystem/Blueprint/Interface/I_IsAlive.Locked`
  ;[0.1554 0.2885 0.2799] Locked(Scanned)
  (`SceneComponent.SetVisibility` (`self.Widget_ScanMark`) true true)
  (`|ExecutionSequence`
    (:`then_0`
      (`KismetSystemLibrary.Delay` (`self.ScanMarkFade`))
      (`self.Unlocked`))
    (:`then_1`
      (`PrimitiveComponent.SetRenderCustomDepth` (`self.Mesh`) true)
      (`PrimitiveComponent.SetRenderCustomDepth` (`self.Glasses`) true)
      (`PrimitiveComponent.SetRenderCustomDepth` (`self.Mask`) true)
      (`PrimitiveComponent.SetRenderCustomDepth` (`self.Hat`) true)
      (`PrimitiveComponent.SetRenderCustomDepth` (`self.Lower`) true)
      (`PrimitiveComponent.SetRenderCustomDepth` (`self.Gloves`) true)
      (`PrimitiveComponent.SetRenderCustomDepth` (`self.Mask2`) true)
      (`KismetSystemLibrary.Delay` 1.5)
      (`PrimitiveComponent.SetRenderCustomDepth` (`self.Mesh`) false)
      (`PrimitiveComponent.SetRenderCustomDepth` (`self.Mask`) false)
      (`PrimitiveComponent.SetRenderCustomDepth` (`self.Hat`) false)
      (`PrimitiveComponent.SetRenderCustomDepth` (`self.Lower`) false)
      (`PrimitiveComponent.SetRenderCustomDepth` (`self.Glasses`) false)
      (`PrimitiveComponent.SetRenderCustomDepth` (`self.Gloves`) false)
      (`PrimitiveComponent.SetRenderCustomDepth` (`self.Mask2`) false))))

(event `CustomEvent`
  ;[0.1554 0.2885 0.2799] Locked(Scanned)
  (`SceneComponent.SetVisibility` (`self.Widget_ScanMark`) false true))

(fn `UserConstructionScript`
  (`parent.UserConstructionScript`)
  (`SkinnedMeshComponent.SetLeaderPoseComponent` (`self.Lower`) (`self.Mesh`) true true)
  (`SkinnedMeshComponent.SetLeaderPoseComponent` (`self.Gloves`) (`self.Mesh`) true true))