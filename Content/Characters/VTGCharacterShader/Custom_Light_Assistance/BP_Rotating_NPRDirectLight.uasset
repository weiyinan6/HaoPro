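; Directional light helper for an NPR character shader that turns to face a target actor and feeds its direction to materials.
; Each tick it smoothly interpolates its rotation toward the target, then writes the light's negated forward vector to the DirectLight parameter of the LightSource material parameter collection.
; The construction script writes the same parameter and adds a child actor component, commented as enabling real-time viewport updates.
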(event `/Game/Characters/VTGCharacterShader/Custom_Light_Assistance/BPI_NPRDirectLight.Light Point To Target`
  (params (Target :type "Object Object Reference")))

(event `self.ReceiveTick`
  (params (DeltaSeconds :type "Float (single-precision)"))
  (bind (_returnvalue_roll _returnvalue_pitch _returnvalue_yaw) (`KismetMathLibrary.BreakRotator` (`KismetMathLibrary.RInterpTo` (`self.K2_GetActorRotation`) (`KismetMathLibrary.FindLookAtRotation` (`self.K2_GetActorLocation`) (`self.K2_GetActorLocation` (`self.Target`))) (`GameplayStatics.GetWorldDeltaSeconds`) 2.0)))
  ;[0.1432 0.1307 0.09071] Rotate Around Target Object
  (`self.K2_SetActorRotation` (`KismetMathLibrary.MakeRotator` _returnvalue_roll _returnvalue_pitch _returnvalue_yaw))
  ;[1 1 1] Casts Forward Ray Upwards to Detect Shadow Casting Objects
  ;;[1 0.4319 0] Make Sure the Paremeter Name is itself
  (`KismetMaterialLibrary.SetVectorParameterValue` "/Game/Characters/VTGCharacterShader/Custom_Light_Assistance/LightSource.LightSource" "DirectLight" (`KismetMathLibrary.Conv_VectorToLinearColor` (* (`SceneComponent.GetForwardVector` (`self.DirectionalLight`)) (-1.0 -1.0 -1.0)))))

(fn `UserConstructionScript`
  ;[1 1 1] Casts Forward Ray Upwards to Detect Shadow Casting Objects
  (`KismetMaterialLibrary.SetVectorParameterValue` "/Game/Characters/VTGCharacterShader/Custom_Light_Assistance/LightSource.LightSource" "DirectLight" (`KismetMathLibrary.Conv_VectorToLinearColor` (* (`SceneComponent.GetForwardVector` (`self.DirectionalLight`)) (-1.0 -1.0 -1.0))))
  ;[1 0.3816 0] BluePrint of Corresponding Mesh (To Add Viewport Real-Time Updates)
  (`AddComponent|NODE_AddChildActorComponent-4`))