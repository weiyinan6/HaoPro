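; BP_StartDialogue is a collision trigger that starts a dialogue row when a Pawn overlaps its collision component.
; By default, pawns with BP_AC_Dialogue start their own dialogue or, if flagged, trigger replicated overhead dialogue on a referenced Pawn.
; With CanOverlapAiStartItsOwnDialogue set, the overlapping pawn's overhead component starts dialogue, and the referenced Pawn's is also attempted.
; IsInDialogue checks prevent restarting active dialogues.
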(event `self.CollisionComponent.OnComponentBeginOverlap`
  (params (OverlappedComponent :type "PrimitiveComponent Object Reference") (OtherActor :type "Actor Object Reference") (OtherComp :type "PrimitiveComponent Object Reference") (OtherBodyIndex :type Integer) (bFromSweep :type Boolean) (SweepResult :type "HitResult Structure (by ref)"))
  (bind _returnvalue (`self.GetComponentByClass` (`self.Pawn`) "/Game/DialogueSystem/Blueprint/ActorComponent/BP_AC_DialogueOverHead.BP_AC_DialogueOverHead_C"))
  ;[1 1 1] Starting a dialogue when the character overlaps in a Box collision
  (bind _aspawn (cast `Pawn` OtherActor))
  (if (not (`self.CanOverlapAiStartItsOwnDialogue?`))
    (bind _returnvalue_2 (`self.GetComponentByClass` _aspawn "/Game/DialogueSystem/Blueprint/ActorComponent/BP_AC_Dialogue.BP_AC_Dialogue_C"))
    (`/Engine/EditorBlueprintResources/StandardMacros.IsValid` _returnvalue_2
      (:`Is Valid`
        (if (`self.OverHeadDialogueByPawnReferance`)
          (`/Engine/EditorBlueprintResources/StandardMacros.IsValid` _returnvalue :!label _label
            (:`Is Valid`
              (if (not (`/Game/DialogueSystem/Blueprint/ActorComponent/BP_AC_DialogueOverHead.IsInDialogue` _returnvalue))
                (`/Game/DialogueSystem/Blueprint/ActorComponent/BP_AC_DialogueOverHead.StartDialogueReplicated` _returnvalue (`self.Row Name`) (`self.Dialogue Actors`)))))
          (elif (not (`/Game/DialogueSystem/Blueprint/ActorComponent/BP_AC_Dialogue.IsInDialogue` _returnvalue_2))
            (`/Game/DialogueSystem/Blueprint/ActorComponent/BP_AC_Dialogue.StartDialogue` _returnvalue_2 (`self.Row Name`) null)))))
    (else
      (bind _returnvalue_3 (`self.GetComponentByClass` _aspawn "/Game/DialogueSystem/Blueprint/ActorComponent/BP_AC_DialogueOverHead.BP_AC_DialogueOverHead_C"))
      (`/Engine/EditorBlueprintResources/StandardMacros.IsValid` _returnvalue_3
        (:`Is Valid`
          (if (`/Game/DialogueSystem/Blueprint/ActorComponent/BP_AC_DialogueOverHead.IsInDialogue` _returnvalue_3)
            (goto _label)
            (else
              (`/Game/DialogueSystem/Blueprint/ActorComponent/BP_AC_DialogueOverHead.StartDialogueReplicated` _returnvalue_3 (`self.Row Name`) (`self.Dialogue Actors`))
              (goto _label))))
        (:`Is Not Valid`
          (goto _label))))))

(fn `UserConstructionScript`)