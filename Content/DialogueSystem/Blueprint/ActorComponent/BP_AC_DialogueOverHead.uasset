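; Actor component that runs replicated overhead dialogue between actors, showing text on each owner's "dialogue"-tagged widget.
; Rows from DT_TextOverHead supply text, sound and speaker index, with server events advancing rows and multicasts updating WBP_TextOverHead.
; Participants' components share an in-dialogue list, used to set busy flags and force-stop everyone together.
; BeginPlay retries until the widget is valid, and a separate event plays character montages.
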(event `self.ReceiveBeginPlay`
  (bind _aswbp_text_over_head (`self.GetWidget`))
  (bind _returnvalue (`self.GetOwner`))
  (bind _output (`|GetArrayItem` (`Actor.GetComponentsByTag` _returnvalue "/Script/UMG.WidgetComponent" "dialogue")))
  ;[1 1 1] get references
  (`/Engine/EditorBlueprintResources/StandardMacros.IsValid` _output
    (:`Is Valid`
      (set `self.WidgetComp` _output)
      (set `self.As Pawn` (cast `Pawn` _returnvalue :!pure true))
      (`/Engine/EditorBlueprintResources/StandardMacros.IsValid` _aswbp_text_over_head :!label _label
        (:`Is Valid`
          (`/Game/DialogueSystem/Blueprint/Widget/WBP_TextOverHead.SetDialogueComp` _aswbp_text_over_head self null)
          (if (`self.IsInDialogue`)
            _))
        (:`Is Not Valid`
          (`KismetSystemLibrary.Delay` 0.1)
          (goto _label))))))

(event `SetRowNameServer`
  (params (RowName :type Name))
  ;[1 0.276 0.276] Replicated
  ;;[1 1 1] Set Row Name
  (set `self.RowName` RowName))

(event `SetTextMulticast`
  (params (RowName :type Name))
  ;[1 0.276 0.276] Replicated
  ;;[1 1 1] Updating text for everyone.
  (`/Game/DialogueSystem/Blueprint/Widget/WBP_TextOverHead.SetTextOnlyClient` (`self.GetWidget`) RowName)
  (`/Engine/EditorBlueprintResources/ActorComponentMacros.Switch Has Authority`
    (:`Authority`
      (bind _returnvalue (`|GetDataTableRow` "/Game/DialogueSystem/Blueprint/DataTable/DT_TextOverHead.DT_TextOverHead" RowName)
        (:`then`
          (set `self.Text` (`.Text_2_9016896247134FC9A7BD4F8F4B425273` (break `/Game/DialogueSystem/Blueprint/Structure/F_TextOverHead` _returnvalue))))))))

(event `ClearTextMulticast`
  ;[1 0.276 0.276] Replicated
  ;;[1 1 1] Clear text for everyone
  (`/Game/DialogueSystem/Blueprint/Widget/WBP_TextOverHead.ClearTextOnlyClient` (`self.GetWidget`)))

(event `SpawnSound`
  (params (Sound :type "SoundBase Object Reference"))
  ;[1 0.276 0.276] Replicated
  ;;[1 1 1] Spawn Sound & Stop Sound
  (bind _sound (`self.Sound`)
    (:`then`
      (`AudioComponent.Stop` _sound)
      (`self.K2_DestroyComponent` _sound))
    (:`else`
      _))
  (bind _returnvalue (`GameplayStatics.SpawnSoundAtLocation` Sound (`Actor.K2_GetActorLocation` (`self.As Pawn`)) (struct) 1.0 1.0 0.0 "/Game/DialogueSystem/Sound/SA_OverHeadDialogue.SA_OverHeadDialogue" null))
  (`/Engine/EditorBlueprintResources/ActorComponentMacros.Switch Has Authority`
    (:`Authority`
      (set `self.Sound` _returnvalue))))

(event `StartDialogueReplicated`
  (params (RowName :type Name) (DialogueActors :type "Array of Actor Object Reference"))
  ;[1 0.276 0.276] Replicated
  ;;[1 1 1] Starting the Dialogue.
  (set `self.RowName` RowName)
  (set `self.Dialogue Actors` DialogueActors)
  (`/Game/DialogueSystem/Blueprint/Widget/WBP_TextOverHead.SetText` (`self.GetWidget`) RowName null)
  (`self.SetTextMulticast` RowName)
  (`self.SetIsInDialogueServer` true)
  (bind _returnvalue (`|GetDataTableRow` "/Game/DialogueSystem/Blueprint/DataTable/DT_TextOverHead.DT_TextOverHead" RowName)
    (:`then`
      (`self.SpawnSound` (`.SpecialSound_31_89BE4A674016219705C71B805592BC99` (break `/Game/DialogueSystem/Blueprint/Structure/F_TextOverHead` _returnvalue))))))

(event `ForceStopDialogueMulti`
  ;[1 0.276 0.276] Replicated
  ;;[1 1 1] force stopping the Dialogue.
  (for _array_element (`self.IsInDialogueComps`)
    (`/Game/DialogueSystem/Blueprint/Widget/WBP_TextOverHead.ForceStopDialogue` (`self.GetWidget` _array_element))
    (`self.SpawnSound` _array_element null)))

(event `ClearTextFromWidgetMulticast`
  (params (Index :type Integer))
  (bind _output (`|GetArrayItem` (`self.Dialogue Actors`) Index))
  ;[1 0.276 0.276] Replicated
  ;;[1 1 1] It is used to clear text from a widget. (It was created to solve clientte bug.)
  (`/Engine/EditorBlueprintResources/StandardMacros.IsValid` _output
    (:`Is Valid`
      (`self.ClearTextMulticast` (`Actor.GetComponentByClass` _output "BP_AC_DialogueOverHead_C")))))

(event `ForceStopDialogueServer`
  ;[1 0.276 0.276] Replicated
  ;;[1 1 1] force stopping the Dialogue.
  (if (not (`KismetArrayLibrary.Array_IsEmpty` (`self.IsInDialogueComps`)))
    (`self.ForceStopDialogueMulti`)
    (`self.SetIsInDialogueToFalse`)
    (`self.DialogueOver` true)
    (`self.SpawnSound` null)
    (`self.ClearIsInDialogueCompsArray`)))

(event `NextRowServer`
  (params (NextRow :type Name) (ClearTextByIndex :type Boolean) (Index :type Integer))
  ;[1 0.276 0.276] Replicated
  ;;[1 1 1] Necessary settings to move to the next row in the dialogue.
  (bind _returnvalue (`|GetDataTableRow` "/Game/DialogueSystem/Blueprint/DataTable/DT_TextOverHead.DT_TextOverHead" NextRow)
    (:`then`
      (if ClearTextByIndex
        (`self.ClearTextFromWidgetMulticast` Index))
      (bind ((`ItIsSelfDialogue_25_1AF048C54AB940A8817ACCB75C942996` _itisselfdialogue) (`DialogueActorIndex_28_72B26E0A4B33E00B026256B0283ADD51` _dialogueactorindex) (`SpecialSound_31_89BE4A674016219705C71B805592BC99` _specialsound)) (break `/Game/DialogueSystem/Blueprint/Structure/F_TextOverHead` _returnvalue))
      (if _itisselfdialogue
        (`/Game/DialogueSystem/Blueprint/Widget/WBP_TextOverHead.SetText` (`self.GetWidget`) NextRow null)
        (`self.SetTextMulticast` NextRow)
        (`self.SpawnSound` _specialsound)
        (else
          (bind _output (`|GetArrayItem` (`self.Dialogue Actors`) _dialogueactorindex))
          (`/Engine/EditorBlueprintResources/StandardMacros.IsValid` _output
            (:`Is Valid`
              (bind _returnvalue_2 (`Actor.GetComponentByClass` _output "BP_AC_DialogueOverHead_C"))
              (`/Game/DialogueSystem/Blueprint/Widget/WBP_TextOverHead.SetText` (`self.GetWidget` _returnvalue_2) NextRow self)
              (`self.ClearTextMulticast`)
              (`self.SetTextMulticast` _returnvalue_2 NextRow)
              (`self.SpawnSound` _specialsound))
            (:`Is Not Valid`
              (`self.SetIsInDialogueServer` false :!label _label_2)
              (`self.ClearTextMulticast`)
              (`self.SpawnSound` null))))))
    (:`RowNotFound`
      (goto _label_2))))

(event `SetIsInDialogueServer`
  (params (IsInDialogue :type Boolean))
  ;[1 0.276 0.276] Replicated
  ;;[1 1 1] Updating the Set Is In Dialogue variable and making the necessary settings accordingly.
  (bind _output_get (set `self.IsInDialogue` IsInDialogue))
  (if _output_get
    (`KismetArrayLibrary.Array_AddUnique` (`self.IsInDialogueComps`) self)
    (`self.SetIsInDialogueVeriableToTrue`)
    (for _array_element (`self.IsInDialogueComps`)
      (if (!= _array_element self)
        (set `/Game/DialogueSystem/Blueprint/ActorComponent/BP_AC_DialogueOverHead.IsInDialogueComps` (`self.IsInDialogueComps`) _array_element)))
    (else
      (`self.SetIsInDialogueToFalse`)
      (`self.DialogueOver` false)
      (`self.ClearIsInDialogueCompsArray`))))

(event `DialogueOver`
  (params (ForceStop :type Boolean))
  ;[1 0.4375 0.4375] Others
  ;;[1 1 1] Dialogue ended event
  (if ForceStop
    _))

(event `DialogueAnim`
  (params (FaceAnim :type "AnimSequence Object Reference") (AnimMontage :type "AnimMontage Object Reference"))
  ;[1 0.4375 0.4375] Others
  ;;[1 1 1] Animation event by dialogue
  (bind _ascharacter (cast `Character` (`self.As Pawn`)))
  (`Character.PlayAnimMontage` _ascharacter AnimMontage 1.0 "None"))

(fn `ClearIsInDialogueCompsArray`
  ;[1 1 1] Clearing the Is In Dialogue Comps variable when the dialogue ends.
  (for _array_element (`self.IsInDialogueComps`)
    (if (!= _array_element self)
      (`KismetArrayLibrary.Array_Clear` (`/Game/DialogueSystem/Blueprint/ActorComponent/BP_AC_DialogueOverHead.IsInDialogueComps` _array_element))))
  (`KismetArrayLibrary.Array_Clear` (`self.IsInDialogueComps`)))

(fn `GetWidget`
  (returns (`AsWBP Text Over Head` :type "/Game/DialogueSystem/Blueprint/Widget/WBP_TextOverHead Object Reference"))
  ;[1 1 1] Get widget reference
  (bind _aswbp_text_over_head (cast `/Game/DialogueSystem/Blueprint/Widget/WBP_TextOverHead` (`WidgetComponent.GetWidget` (`self.WidgetComp`))))
  (return _aswbp_text_over_head))

(fn `SetIsInDialogueToFalse`
  ;[1 1 1] Setting the Is In Dialogue and Replicated Dialogue variables to false when the dialogue ends
  (for _array_element (`self.IsInDialogueComps`)
    (set `/Game/DialogueSystem/Blueprint/ActorComponent/BP_AC_DialogueOverHead.IsInDialogue` false _array_element)))

(fn `SetIsInDialogueVeriableToTrue`
  ;[1 1 1] When the dialogue starts, reference other characters related to the dialogue with the actor tag.
  (for _array_element (`self.Dialogue Actors`)
    (`/Engine/EditorBlueprintResources/StandardMacros.IsValid` _array_element
      (:`Is Valid`
        (bind _returnvalue (`Actor.GetComponentByClass` _array_element "BP_AC_DialogueOverHead_C"))
        (`KismetArrayLibrary.Array_AddUnique` (`self.IsInDialogueComps`) _returnvalue)
        (set `/Game/DialogueSystem/Blueprint/ActorComponent/BP_AC_DialogueOverHead.IsInDialogue` true _returnvalue)))))