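; Player pawn component that runs NPC dialogue, opening the main dialogue widget from a DT_Dialogue row and switching input by dialogue type.
; In face-to-face dialogue, Tick turns both actors toward each other through server rotation events, and FocusCamera blends to tagged child-actor cameras.
; It also relays montages to pawn and NPC, drives the pawn's overhead text widget, and restores input and view on close.
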(event `SetActorRotationServer`
  (params (Target :type "Actor Object Reference") (NewRotation :type "Rotator Structure"))
  ;[1 1 1] Update the actor's rotation.
  (`/Engine/EditorBlueprintResources/StandardMacros.IsValid` Target
    (:`Is Valid`
      (`Actor.K2_SetActorRotation` Target NewRotation false))))

(event `SetActorRotationOwningClient`
  (params (Target :type "Actor Object Reference") (NewRotation :type "Rotator Structure"))
  ;[1 1 1] Update the actor's rotation.
  (`Actor.K2_SetActorRotation` Target NewRotation false))

(event `SetIsInDialogueFasle`
  (bind _dialogueactor (`self.DialogueActor`))
  ;[1 1 1] Setting the Dialogue Variable to false.
  (`/Engine/EditorBlueprintResources/StandardMacros.IsValid` _dialogueactor
    (:`Is Valid`
      (message `/Game/DialogueSystem/Blueprint/Interface/BP_I_Dialogue.SetIsInDialogue` _dialogueactor false))))

(event `UpdateInputsToGame`
  (bind _asplayer_controller (cast `PlayerController` (`Pawn.GetController` (`self.As Pawn`)) :!pure true))
  ;[1 1 1] Setting Input Mode to the game.
  (set `PlayerController.bShowMouseCursor` false _asplayer_controller)
  (`WidgetBlueprintLibrary.SetInputMode_GameOnly` _asplayer_controller)
  (`WidgetBlueprintLibrary.SetFocusToGameViewport`)
  (switch `/Game/DialogueSystem/Blueprint/Enum/E_DialogueType` (`self.Dialogue Type`)
    (:`NewEnumerator0`
      _)
    (:`NewEnumerator2`
      _))
  (`Actor.EnableInput` (`self.As Pawn`) _asplayer_controller))

(event `SetDialogueType`
  (params (DialogueType :type "/Game/DialogueSystem/Blueprint/Enum/E_DialogueType Enum" :default "NewEnumerator0"))
  ;[1 1 1] Set Veriables
  (set `self.Dialogue Type` DialogueType))

(event `UpdateInputsToWidget`
  (params (DialogueType :type "/Game/DialogueSystem/Blueprint/Enum/E_DialogueType Enum" :default "NewEnumerator0"))
  (bind _asplayer_controller (cast `PlayerController` (`Pawn.GetController` (`self.As Pawn`)) :!pure true))
  ;[1 1 1] Setting Input Mode to the viewport
  (switch `/Game/DialogueSystem/Blueprint/Enum/E_DialogueType` DialogueType
    (:`NewEnumerator0`
      (`Actor.DisableInput` (`self.As Pawn`) _asplayer_controller)
      (`WidgetBlueprintLibrary.SetInputMode_UIOnlyEx` _asplayer_controller (`self.MainDialogue`)))))

(event `SetViewTargetWithBlendOwningClient`
  ;[1 1 1] Updating the camera to pawn with Set View Target with Blend.
  (`PlayerController.SetViewTargetWithBlend` (cast `PlayerController` (`Pawn.GetController` (`self.As Pawn`)) :!pure true) (`self.As Pawn`) 0.0 "VTBlend_Linear" 0.0 false))

(event `ForceStopDialogueServer`
  (params (Target :type "/Game/DialogueSystem/Blueprint/ActorComponent/BP_AC_DialogueOverHead Object Reference"))
  ;[1 1 1] Force stop Over Head dialogue
  (`/Game/DialogueSystem/Blueprint/ActorComponent/BP_AC_DialogueOverHead.ForceStopDialogueServer` Target))

(event `SetValidFocusCamera`
  (params (ValidFocusCamera :type Boolean))
  ;[1 1 1] Set Veriables
  (set `self.ValidFocusCamera` ValidFocusCamera))

(event `CloseWidget`
  ;[1 1 1] Widget close event
  (`self.SetIsInDialogue` false)
  (`self.SetIsInDialogueFasle`)
  (`self.SetDialogueActor` null)
  (`Widget.RemoveFromParent` (`self.MainDialogue`))
  (`self.UpdateInputsToGame`))

(event `SetIsInDialogue`
  (params (IsInDialogue :type Boolean))
  ;[1 1 1] Set Is In Dialogue Veriable
  (bind _output_get (set `self.IsInDialogue` IsInDialogue))
  (if _output_get
    _
    (elif (`self.ValidFocusCamera`)
      (`self.SetViewTargetWithBlendOwningClient`)
      (`self.SetValidFocusCamera` false))))

(event `SetDialogueActor`
  (params (DialogueActor :type "Actor Object Reference"))
  ;[1 1 1] Update Dialogue actor
  (bind _output_get (set `self.DialogueActor` DialogueActor))
  (`self.DialogueActor`
    (:`then`
      (`/Engine/EditorBlueprintResources/StandardMacros.IsValid` _output_get
        (:`Is Valid`
          (message `/Game/DialogueSystem/Blueprint/Interface/BP_I_Dialogue.SetIsInDialogue` _output_get true))
        (:`Is Not Valid`)))
    (:`else`)))

(event `StartDialogue`
  (params (RowName :type Name) (Actor :type "Actor Object Reference"))
  (bind _returnvalue (`Actor.GetComponentByClass` Actor "/Game/DialogueSystem/Blueprint/ActorComponent/BP_AC_DialogueOverHead.BP_AC_DialogueOverHead_C"))
  ;[1 1 1] Starting the dialog and making the necessary settings. (Adding the widget to the viewport, updating variables, editing input, etc.)
  (bind _returnvalue_2 (`|GetDataTableRow` "/Game/DialogueSystem/Blueprint/DataTable/DT_Dialogue.DT_Dialogue" RowName)
    (:`then`
      (`self.SetDialogueActor` Actor)
      (`/Engine/EditorBlueprintResources/StandardMacros.IsValid` Actor
        (:`Is Valid`
          (`/Engine/EditorBlueprintResources/StandardMacros.IsValid` _returnvalue
            (:`Is Valid`
              (`self.ForceStopDialogueServer` _returnvalue))
            (:`Is Not Valid`
              _)))
        (:`Is Not Valid`
          _))
      (`/Game/DialogueSystem/Blueprint/Widget/WBP_MainDialogue.StartDialogue` (`self.MainDialogue`) RowName)
      (`UserWidget.AddToViewport` (`self.MainDialogue`) 0)
      (`self.SetIsInDialogue` true)
      (bind ((`DialogueType_85_6967DC87423A5C440C858AB5AF289266` _dialoguetype)) (break `/Game/DialogueSystem/Blueprint/Structure/F_Dialogue` _returnvalue_2))
      (`self.SetDialogueType` _dialoguetype)
      (`self.UpdateInputsToWidget` _dialoguetype))))

(event `self.ReceiveTick`
  (params (DeltaSeconds :type "Float (single-precision)"))
  (bind _as_pawn (`self.As Pawn`))
  (bind _returnvalue (`KismetMathLibrary.FindLookAtRotation` (`Actor.K2_GetActorLocation` (`self.DialogueActor`)) (`Actor.K2_GetActorLocation` (`self.As Pawn`))))
  (bind _returnvalue_2 (`KismetMathLibrary.MakeRotator` 0.0 0.0 (.yaw (`KismetMathLibrary.FindLookAtRotation` (`Actor.K2_GetActorLocation` (`self.As Pawn`)) (`Actor.K2_GetActorLocation` (`self.DialogueActor`))))))
  (bind _returnvalue_3 (`KismetMathLibrary.RInterpTo` (`Actor.K2_GetActorRotation` (`self.As Pawn`)) _returnvalue_2 (`GameplayStatics.GetWorldDeltaSeconds`) (`KismetMathLibrary.SelectFloat` 5000.0 10.0 (`self.QuickRotation`))))
  (bind _returnvalue_4 (`KismetMathLibrary.RInterpTo` (`Actor.K2_GetActorRotation` (`self.DialogueActor`)) (`KismetMathLibrary.MakeRotator` 0.0 0.0 (.yaw _returnvalue)) (`GameplayStatics.GetWorldDeltaSeconds`) (`KismetMathLibrary.SelectFloat` 5000.0 10.0 (`self.QuickRotation`))))
  ;[1 1 1] Update rotation values ​​of actors
  (`self.DialogueActor`
    (:`then`
      (if (not (`self.DisableRotation`))
        (switch `/Game/DialogueSystem/Blueprint/Enum/E_DialogueType` (`self.Dialogue Type`)
          (:`NewEnumerator0`
            (if (not (== (`Actor.K2_GetActorRotation` (`self.DialogueActor`)) _returnvalue_4 :`ErrorTolerance` 0.1))
              (if (`self.QuickRotation`)
                (`self.SetActorRotationServer` (`self.DialogueActor`) _returnvalue)
                (else
                  (`self.SetActorRotationServer` (`self.DialogueActor`) _returnvalue_4)))
              (if (not (== (`Actor.K2_GetActorRotation` (`self.As Pawn`)) _returnvalue_3 :`ErrorTolerance` 0.1))
                (if (`self.QuickRotation`) :!label _label
                  (`self.SetActorRotationServer` (`self.As Pawn`) _returnvalue_2)
                  (else
                    (`self.SetActorRotationServer` _as_pawn _returnvalue_3)
                    (`self.SetActorRotationOwningClient` _as_pawn _returnvalue_3))))
              (else
                (goto _label)))))))
    (:`else`)))

(event `self.ReceiveBeginPlay`
  (bind _aswbp_text_over_head (`self.GetWidget`))
  (bind _returnvalue (`self.GetOwner`))
  (bind _output (`|GetArrayItem` (`Actor.GetComponentsByTag` _returnvalue "/Script/UMG.WidgetComponent" "dialogue")))
  (bind _output_2 (`|GetArrayItem` (`Actor.GetComponentsByTag` (`self.As Pawn`) "/Script/Engine.ChildActorComponent" "dialogue")))
  ;[1 1 1] Creating the dialogue widget
  (`|ExecutionSequence`
    (:`then_0`
      (set `self.As Pawn` (cast `Pawn` (`self.GetOwner`) :!pure true))
      (bind _returnvalue_2 (`|CreateWidget` "/Game/DialogueSystem/Blueprint/Widget/WBP_MainDialogue.WBP_MainDialogue_C"))
      (bind _output_get (set `self.MainDialogue` _returnvalue_2))
      (if (not (and (`KismetSystemLibrary.IsDedicatedServer`) (`Actor.HasAuthority` (`self.GetOwner`))))
        (`UserWidget.AddToViewport` _output_get 0)
        (`Widget.RemoveFromParent` _output_get)))
    (:`then_1`
      (`/Engine/EditorBlueprintResources/StandardMacros.IsValid` _output
        (:`Is Valid`
          (set `self.WidgetComp` _output)
          (set `self.As Pawn` (cast `Pawn` _returnvalue :!pure true))
          (`/Engine/EditorBlueprintResources/StandardMacros.IsValid` _aswbp_text_over_head :!label _label_2
            (:`Is Valid`
              (`/Game/DialogueSystem/Blueprint/Widget/WBP_TextOverHead.SetDialogueComp` _aswbp_text_over_head null self)
              (if (`self.OverHeadDialogue`)
                (`TextBlock.SetText` (`/Game/DialogueSystem/Blueprint/Widget/WBP_TextOverHead.TextBlock` _aswbp_text_over_head) (`self.Text`))))
            (:`Is Not Valid`
              (`KismetSystemLibrary.Delay` 0.1)
              (goto _label_2))))))
    (:`then_2`
      (`/Engine/EditorBlueprintResources/StandardMacros.IsValid` _output_2
        (:`Is Valid`
          (set `self.CameraChildActor` _output_2))))))

(event `DialogueAnim`
  (params (FaceAnim :type "AnimSequence Object Reference") (AnimMontage :type "AnimMontage Object Reference"))
  ;[1 0 0] Our Character, It is used to play the animation specified in the data table for our character.
  (bind _ascharacter (cast `Character` (`self.As Pawn`)))
  (`Character.PlayAnimMontage` _ascharacter AnimMontage 1.0 "None"))

(event `OverHeadTextServer`
  (params (OverHeadText :type Text) (Duration :type "Float (single-precision)" :default 3.0))
  ;[1 1 1] Over Head Text system (Text update, sending information to clients, Force stopping text.)
  (`/Engine/EditorBlueprintResources/StandardMacros.IsValid` (`self.WidgetComp`)
    (:`Is Valid`
      (`/Game/DialogueSystem/Blueprint/Widget/WBP_TextOverHead.SetTextForController` (`self.GetWidget`) OverHeadText Duration)
      (`self.OverHeadTextClientOnly` OverHeadText)
      (set `self.Text` OverHeadText)
      (set `self.OverHeadDialogue` true))))

(event `OverHeadTextClientOnly`
  (params (OverHeadText :type Text))
  ;[1 1 1] Over Head Text system (Text update, sending information to clients, Force stopping text.)
  (`/Game/DialogueSystem/Blueprint/Widget/WBP_TextOverHead.SetTextOnlyClientForController` (`self.GetWidget`) OverHeadText))

(event `DialogueAnimNPC`
  (params (FaceAnim :type "AnimSequence Object Reference") (AnimMontage :type "AnimMontage Object Reference"))
  ;[1 0 0] NPC, It is used to play animations for the character entered into the dialogue.
  (bind _dialogueactor (`self.DialogueActor`)
    (:`then`
      (message `/Game/DialogueSystem/Blueprint/Interface/BP_I_Dialogue.DialogueAnim` _dialogueactor FaceAnim AnimMontage))
    (:`else`)))

(event `OverHeadClearTextServer`
  ;[1 1 1] Over Head Text system (Text update, sending information to clients, Force stopping text.)
  (`self.OverHeadClearTextMulti`))

(event `OverHeadClearTextMulti`
  ;[1 1 1] Over Head Text system (Text update, sending information to clients, Force stopping text.)
  (`/Game/DialogueSystem/Blueprint/Widget/WBP_TextOverHead.ForceStopDialogue` (`self.GetWidget`)))

(event `FocusCamera`
  (params (Speaker :type "/Game/DialogueSystem/Blueprint/Enum/E_SpeakerForFocusCamera Enum" :default "NewEnumerator0"))
  (bind _childactor (`ChildActorComponent.ChildActor` (`self.CameraChildActor`)))
  (bind _asplayer_controller (cast `PlayerController` (`Pawn.GetController` (`self.As Pawn`)) :!pure true))
  ;[1 1 1] In the Face to Face dialogue system, focusing the camera on the actors.
  (switch `/Game/DialogueSystem/Blueprint/Enum/E_SpeakerForFocusCamera` Speaker
    (:`NewEnumerator0`
      (`/Engine/EditorBlueprintResources/StandardMacros.IsValid` _childactor
        (:`Is Valid`
          (`PlayerController.SetViewTargetWithBlend` _asplayer_controller _childactor 0.0 "VTBlend_Linear" 0.0 false))))
    (:`NewEnumerator1`
      (bind _dialogueactor (`self.DialogueActor`)
        (:`then`
          (bind _output (`|GetArrayItem` (`Actor.GetComponentsByTag` _dialogueactor "/Script/Engine.ChildActorComponent" "dialogue")))
          (`/Engine/EditorBlueprintResources/StandardMacros.IsValid` _output
            (:`Is Valid`
              (`PlayerController.SetViewTargetWithBlend` _asplayer_controller (`ChildActorComponent.ChildActor` _output) 0.0 "VTBlend_Linear" 0.0 false))))
        (:`else`))))
  (`self.SetValidFocusCamera` true))

(event `SelectedOption`
  (params (Option :type Name))
  ;[1 0 0] This is triggered when any option is selected in the dialogue.
  (switch `name` Option
    (:`Quit`
      (`KismetSystemLibrary.QuitGame` (`GameplayStatics.GetPlayerController` 0) "Quit"))))

(fn `DisableInputAndFocusWidget`
  (bind _asplayer_controller (cast `PlayerController` (`Pawn.GetController` (`self.As Pawn`)) :!pure true))
  ;[1 1 1] In the free movement dialogue type, it is triggered when the option appears and updates the input.
  (`Actor.DisableInput` (`self.As Pawn`) _asplayer_controller)
  (`WidgetBlueprintLibrary.SetInputMode_UIOnlyEx` _asplayer_controller null))

(fn `EnableInputAndFocusGame`
  (bind _asplayer_controller (cast `PlayerController` (`Pawn.GetController` (`self.As Pawn`)) :!pure true))
  ;[1 1 1] In the free movement dialogue type, it is triggered when the option appears and updates the input.
  (`WidgetBlueprintLibrary.SetInputMode_GameOnly` _asplayer_controller)
  (`WidgetBlueprintLibrary.SetFocusToGameViewport`)
  (`Actor.EnableInput` (`self.As Pawn`) _asplayer_controller))

(fn `GetWidget`
  (returns (`AsWBP Text Over Head` :type "/Game/DialogueSystem/Blueprint/Widget/WBP_TextOverHead Object Reference"))
  ;[1 1 1] Get widget reference
  (bind _aswbp_text_over_head (cast `/Game/DialogueSystem/Blueprint/Widget/WBP_TextOverHead` (`WidgetComponent.GetWidget` (`self.WidgetComp`))))
  (return _aswbp_text_over_head))