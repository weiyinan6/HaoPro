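; Bullet projectile in the AI behavior system that damages what it hits and alerts AI perception.
; It limits its lifespan on begin play and destroys itself on any blocking hit, doing nothing else if it hit its owner.
; Other hits spawn flesh or metal impact effects and sound depending on whether a Character was struck, then apply point damage.
; It also reports damage and noise events at the impact point for AI damage and hearing senses.
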(event `self.ReceiveBeginPlay`
  ;[1 0.6706 0.2488] Beginplay
  ;;[1 1 1] Set lifespan
  (`self.SetLifeSpan` (`self.Lifespan`)))

(event `self.ReceiveHit`
  (params (MyComp :type "PrimitiveComponent Object Reference") (Other :type "Actor Object Reference") (OtherComp :type "PrimitiveComponent Object Reference") (bSelfMoved :type Boolean) (HitLocation :type "Vector Structure") (HitNormal :type "Vector Structure") (NormalImpulse :type "Vector Structure") (Hit :type "HitResult Structure (by ref)"))
  (bind (_bblockinghit _binitialoverlap _time _distance _location _impactpoint _normal _impactnormal _physmat _hitactor) (`GameplayStatics.BreakHitResult` Hit))
  (bind _returnvalue (`self.GetOwner`))
  ;[1 0.6706 0.2488] On Hit
  (if _bblockinghit
    (if (!= _hitactor (`self.GetOwner`))
      (cast `Character` _hitactor
        (:`then`
          (`GameplayStatics.SpawnEmitterAtLocation` "/Game/AIBehaviorSystem/Demo/Particles/P_body_bullet_impact.P_body_bullet_impact" _impactpoint)
          (`GameplayStatics.PlaySoundAtLocation` "/Game/AIBehaviorSystem/Demo/Audio/Impact/ImpactFlesh.ImpactFlesh" _impactpoint (struct) 1.0 1.0 0.0 null null null null))
        (:`CastFailed`
          (`GameplayStatics.SpawnEmitterAtLocation` "/Game/AIBehaviorSystem/Demo/Particles/P_Impact.P_Impact" _impactpoint (struct) (0.5 0.5 0.5))
          (`GameplayStatics.PlaySoundAtLocation` "/Game/AIBehaviorSystem/Demo/Audio/Impact/ImpactMetal.ImpactMetal" _impactpoint (struct) 1.0 1.0 0.0 null null null null)))
      (`GameplayStatics.ApplyPointDamage` _hitactor (`self.Damage`) (`KismetMathLibrary.GetDirectionUnitVector` (`self.K2_GetActorLocation`) (`self.K2_GetActorLocation` _hitactor)) Hit null _returnvalue)
      (`AISense_Damage.ReportDamageEvent` _hitactor _returnvalue (`self.Damage`) _impactpoint) ; Report Damage for AI Damage Sense
      (`AISense_Hearing.ReportNoiseEvent` _impactpoint 1.0 _returnvalue (`self.NoiseMaxRange`)) ; Report Noise for AI Hearing Sense
      (`self.K2_DestroyActor`)
      (else
        (`self.K2_DestroyActor`)))))

(fn `UserConstructionScript`)