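; Anim notify state "Hit Collision" that switches a character's hit collision on for the span of an animation window.
; On begin it tells the owner's BP_CollisionComponent to enable the configured CollisionPart, and on end it disables collision.
; Only the locally controlled character acts, calling the component directly with authority or through its Server functions otherwise.
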(fn `GetNotifyName`
  (returns (ReturnValue :type String))
  (return "Hit Collision"))

(fn `Received_NotifyBegin`
  (params (MeshComp :type "SkeletalMeshComponent Object Reference") (Animation :type "AnimSequenceBase Object Reference") (TotalDuration :type "Float (single-precision)") (EventReference :type "AnimNotifyEventReference Structure (by ref)"))
  (returns (ReturnValue :type Boolean))
  (bind _returnvalue (`ActorComponent.GetOwner` MeshComp))
  (bind _collision_part (`self.Collision Part`))
  (bind _returnvalue_2 (`Actor.GetComponentByClass` _returnvalue "/Game/AIBehaviorSystem/Blueprint/Component/BP_CollisionComponent.BP_CollisionComponent_C"))
  (bind _ascharacter (cast `Character` _returnvalue))
  (if (`Pawn.IsLocallyControlled` _ascharacter)
    (`/Engine/EditorBlueprintResources/StandardMacros.IsValid` _returnvalue_2
      (:`Is Valid`
        (if (`Actor.HasAuthority` _ascharacter)
          (`/Game/AIBehaviorSystem/Blueprint/Component/BP_CollisionComponent.EnableCollision` _returnvalue_2 _collision_part)
          (else
            (`/Game/AIBehaviorSystem/Blueprint/Component/BP_CollisionComponent.Server_EnableCollision` _returnvalue_2 _collision_part)))
        (return true))
      (:`Is Not Valid`
        (return false)))))

(fn `Received_NotifyEnd`
  (params (MeshComp :type "SkeletalMeshComponent Object Reference") (Animation :type "AnimSequenceBase Object Reference") (EventReference :type "AnimNotifyEventReference Structure (by ref)"))
  (returns (ReturnValue :type Boolean))
  (bind _returnvalue (`ActorComponent.GetOwner` MeshComp))
  (bind _returnvalue_2 (`Actor.GetComponentByClass` _returnvalue "/Game/AIBehaviorSystem/Blueprint/Component/BP_CollisionComponent.BP_CollisionComponent_C"))
  (bind _ascharacter (cast `Character` _returnvalue))
  (if (`Pawn.IsLocallyControlled` _ascharacter)
    (`/Engine/EditorBlueprintResources/StandardMacros.IsValid` _returnvalue_2
      (:`Is Valid`
        (if (`Actor.HasAuthority` _ascharacter)
          (`/Game/AIBehaviorSystem/Blueprint/Component/BP_CollisionComponent.DisableCollision` _returnvalue_2)
          (else
            (`/Game/AIBehaviorSystem/Blueprint/Component/BP_CollisionComponent.Server_DisableCollision` _returnvalue_2)))
        (return true))
      (:`Is Not Valid`
        (return false)))))