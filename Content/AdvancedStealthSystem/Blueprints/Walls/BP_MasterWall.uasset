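; BP_MasterWall is a wall Blueprint in the stealth system that tracks whether a ThirdPersonCharacter is inside its Box1 volume.
; A looping timer started on BeginPlay polls the box's overlaps every fraction of a second and sets the IsOpposite flag accordingly.
; A leftover-looking debug print shows the flag only for the instance named BP_InvisibleWall3.
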(event `self.ReceiveBeginPlay`
  (`KismetSystemLibrary.K2_SetTimer` null "UpdateOpposite" 0.05 true))

(event `UpdateOpposite`
  (if (> (`KismetArrayLibrary.Array_Length` (`PrimitiveComponent.GetOverlappingActors` (`self.Box1`) "/Game/AdvancedStealthSystem/ThirdPersonBP/Blueprints/ThirdPersonCharacter.ThirdPersonCharacter_C")) 0)
    (set `self.isOpposite?` true)
    (if (`KismetStringLibrary.EqualEqual_StrStr` (`KismetSystemLibrary.GetDisplayName` self) "BP_InvisibleWall3")
      (`KismetSystemLibrary.PrintString` (`KismetStringLibrary.Conv_BoolToString` (`self.isOpposite?`))))
    (else
      (set `self.isOpposite?` false))))

(fn `UserConstructionScript`)