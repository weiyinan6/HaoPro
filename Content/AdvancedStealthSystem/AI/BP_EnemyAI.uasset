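; Stealth-game enemy AI character that can hear the player, be knocked out, and then be grabbed as a body.
; A perception update sets HeardPlayer for one second.
; KnockDownCollider registers the living enemy on the player and shows a camera-facing prompt widget; KnockDown runs once, unpossessing it and launching it into ragdoll.
; Once dead, the Sphere overlap offers it to the player as EnemyToGrab.
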(event `self.AIPerception.OnPerceptionUpdated`
  (params (UpdatedActors :type "Array of Actor Object Reference (by ref)"))
  ;[1 1 1] Handles hearing player's noises
  (set `self.heardPlayer?` true)
  (`KismetSystemLibrary.Delay` 1.0)
  (set `self.heardPlayer?` false))

(event `KnockDown`
  (bind _mesh (`self.Mesh`))
  ;[1 1 1] Knocks down enemy
  (`/Engine/EditorBlueprintResources/StandardMacros.DoOnce` false
    (:`Completed`
      (`self.SetActorTickEnabled` false)
      (`Controller.UnPossess` (`self.GetController`))
      (`PrimitiveComponent.SetSimulatePhysics` (`self.Mesh`) true)
      (`PrimitiveComponent.AddForce` _mesh (+ (`SceneComponent.GetSocketLocation` _mesh "head") (* (`self.GetActorForwardVector`) 500000.0)) "head" false)
      (set `self.isDead?` true)
      (`PrimitiveComponent.SetCollisionEnabled` (`self.CapsuleComponent`) "NoCollision")
      (`SceneComponent.SetVisibility` (`self.KnockDownWidget`) false false))))

(event `self.KnockDownCollider.OnComponentBeginOverlap`
  (params (OverlappedComponent :type "PrimitiveComponent Object Reference") (OtherActor :type "Actor Object Reference") (OtherComp :type "PrimitiveComponent Object Reference") (OtherBodyIndex :type Integer) (bFromSweep :type Boolean) (SweepResult :type "HitResult Structure (by ref)"))
  ;[1 1 1] Adds enemy to knock down actor of player
  (if (not (`self.isDead?`))
    (bind _asthird_person_character (cast `/Game/AdvancedStealthSystem/ThirdPersonBP/Blueprints/ThirdPersonCharacter` OtherActor))
    (set `/Game/AdvancedStealthSystem/ThirdPersonBP/Blueprints/ThirdPersonCharacter.knockDownEnemy` self _asthird_person_character)
    (`SceneComponent.SetVisibility` (`self.KnockDownWidget`) true false)))

(event `self.ReceiveTick`
  (params (DeltaSeconds :type "Float (single-precision)"))
  (bind _knockdownwidget (`self.KnockDownWidget`))
  ;[1 1 1] Rotates knock down widget to player
  (if (`SceneComponent.bVisible` (`self.KnockDownWidget`))
    (`SceneComponent.K2_SetWorldRotation` _knockdownwidget (`KismetMathLibrary.FindLookAtRotation` (`SceneComponent.K2_GetComponentLocation` _knockdownwidget) (`self.K2_GetActorLocation` (`GameplayStatics.GetPlayerCameraManager` 0))) false false)))

(event `self.KnockDownCollider.OnComponentEndOverlap`
  (params (OverlappedComponent :type "PrimitiveComponent Object Reference") (OtherActor :type "Actor Object Reference") (OtherComp :type "PrimitiveComponent Object Reference") (OtherBodyIndex :type Integer))
  ;[1 1 1] Removes enemy from knock down actor of player
  (if (not (`self.isDead?`))
    (bind _asthird_person_character (cast `/Game/AdvancedStealthSystem/ThirdPersonBP/Blueprints/ThirdPersonCharacter` OtherActor))
    (set `/Game/AdvancedStealthSystem/ThirdPersonBP/Blueprints/ThirdPersonCharacter.knockDownEnemy` null _asthird_person_character)
    (`SceneComponent.SetVisibility` (`self.KnockDownWidget`) false false)))

(event `self.Sphere.OnComponentBeginOverlap`
  (params (OverlappedComponent :type "PrimitiveComponent Object Reference") (OtherActor :type "Actor Object Reference") (OtherComp :type "PrimitiveComponent Object Reference") (OtherBodyIndex :type Integer) (bFromSweep :type Boolean) (SweepResult :type "HitResult Structure (by ref)"))
  (bind _returnvalue (`GameplayStatics.GetPlayerCharacter` 0))
  ;[1 1 1] Adds enemy to player grab
  (if (and (== OtherActor _returnvalue) (`self.isDead?`))
    (set `/Game/AdvancedStealthSystem/ThirdPersonBP/Blueprints/ThirdPersonCharacter.enemyToGrab` self (cast `/Game/AdvancedStealthSystem/ThirdPersonBP/Blueprints/ThirdPersonCharacter` _returnvalue :!pure true))))

(event `self.Sphere.OnComponentEndOverlap`
  (params (OverlappedComponent :type "PrimitiveComponent Object Reference") (OtherActor :type "Actor Object Reference") (OtherComp :type "PrimitiveComponent Object Reference") (OtherBodyIndex :type Integer))
  (bind _returnvalue (`GameplayStatics.GetPlayerCharacter` 0))
  (bind _asthird_person_character (cast `/Game/AdvancedStealthSystem/ThirdPersonBP/Blueprints/ThirdPersonCharacter` _returnvalue :!pure true))
  ;[1 1 1] Removes enemy from player grab
  (if (== OtherActor _returnvalue)
    (if (== (`/Game/AdvancedStealthSystem/ThirdPersonBP/Blueprints/ThirdPersonCharacter.enemyToGrab` _asthird_person_character) self)
      (set `/Game/AdvancedStealthSystem/ThirdPersonBP/Blueprints/ThirdPersonCharacter.enemyToGrab` null _asthird_person_character))))

(fn `UserConstructionScript`)